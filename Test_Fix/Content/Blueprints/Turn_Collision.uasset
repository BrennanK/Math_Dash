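; Turn trigger actor that swings the third-person player 90 degrees left or right when they overlap its box, then destroys itself.
; Overlap caches the player's actor and control rotations and starts a looping timer at frame delta that advances LerpAlpha over LerpTime.
; Each step lerps both rotations by the LeftOrRight setting and nudges the player along a slerped unit vector.
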(event `self.Box.OnComponentBeginOverlap`
  (params (OverlappedComponent :type "PrimitiveComponent Object Reference") (OtherActor :type "Actor Object Reference") (OtherComp :type "PrimitiveComponent Object Reference") (OtherBodyIndex :type Integer) (bFromSweep :type Boolean) (SweepResult :type "HitResult Structure (by ref)"))
  (bind _asbp_third_person_character (cast `/Game/ThirdPerson/Blueprints/BP_ThirdPersonCharacter` OtherActor))
  (set `self.Player ref` _asbp_third_person_character)
  (set `self.Original Player Rotation` (`self.K2_GetActorRotation` _asbp_third_person_character))
  (set `self.Original Controller Rotation` (`Controller.GetControlRotation` (`Pawn.GetController` _asbp_third_person_character)))
  (bind _returnvalue (`KismetSystemLibrary.K2_SetTimer` null "Lerp Value" (`GameplayStatics.GetWorldDeltaSeconds`) true)))

(event `Reset Timer`
  (`KismetSystemLibrary.K2_ClearAndInvalidateTimerHandle` (stale `self.Box.OnComponentBeginOverlap` _returnvalue))
  (set `self.Lerp Alpha` 0.0))

(event `Lerp Value`
  (if (>= (`self.Lerp Alpha`) 1.0)
    (set `self.Lerp Alpha` 1.0)
    (switch `/Game/Blueprints/Turn_Directions` (`self.Left Or Right`)
      (:`NewEnumerator0`
        (`self.Rotate and Turn Left`))
      (:`NewEnumerator1`
        (`self.Rotate and Turn Right`)))
    (`self.Reset Timer`)
    (`self.K2_DestroyActor`)
    (else
      (switch `/Game/Blueprints/Turn_Directions` (`self.Left Or Right`)
        (:`NewEnumerator0`
          (`self.Rotate and Turn Left`))
        (:`NewEnumerator1`
          (`self.Rotate and Turn Right`)))
      (set `self.Lerp Alpha` (+ (`self.Lerp Alpha`) (/ (`GameplayStatics.GetWorldDeltaSeconds`) (`self.Lerp Time`)))))))

(fn `Rotate and Turn Left`
  (bind _player_ref (`self.Player ref`))
  (bind _original_player_rotation (`self.Original Player Rotation`))
  (bind _player_ref_2 (`self.Player ref`))
  (bind _original_controller_rotation (`self.Original Controller Rotation`))
  (`self.K2_SetActorRotation` _player_ref_2 (`KismetMathLibrary.RLerp` _original_player_rotation (`KismetMathLibrary.MakeRotator` (.roll _original_player_rotation) (.pitch _original_player_rotation) (- (.yaw _original_player_rotation) 90.0)) (`self.Lerp Alpha`)) false)
  (`Controller.SetControlRotation` (`Pawn.GetController` _player_ref_2) (`KismetMathLibrary.RLerp` _original_controller_rotation (`KismetMathLibrary.MakeRotator` (.roll _original_controller_rotation) (.pitch _original_controller_rotation) (- (.yaw _original_controller_rotation) 90.0)) (`self.Lerp Alpha`)))
  (`self.K2_SetActorLocation` _player_ref (+ (`KismetMathLibrary.Vector_SlerpNormals` (`KismetMathLibrary.Normal` (`self.Original Actor Location`)) (`KismetMathLibrary.Normal` (+ (`self.K2_GetActorLocation`) (* (`self.GetActorRightVector`) -100.0))) (`self.Lerp Alpha`)) (`self.K2_GetActorLocation` _player_ref)) false false))

(fn `Rotate and Turn Right`
  (bind _original_player_rotation (`self.Original Player Rotation`))
  (bind _player_ref (`self.Player ref`))
  (bind _player_ref_2 (`self.Player ref`))
  (bind _original_controller_rotation (`self.Original Controller Rotation`))
  (`self.K2_SetActorRotation` _player_ref_2 (`KismetMathLibrary.RLerp` _original_player_rotation (`KismetMathLibrary.MakeRotator` (.roll _original_player_rotation) (.pitch _original_player_rotation) (+ (.yaw _original_player_rotation) 90.0)) (`self.Lerp Alpha`)) false)
  (`Controller.SetControlRotation` (`Pawn.GetController` _player_ref_2) (`KismetMathLibrary.RLerp` _original_controller_rotation (`KismetMathLibrary.MakeRotator` (.roll _original_controller_rotation) (.pitch _original_controller_rotation) (+ (.yaw _original_controller_rotation) 90.0)) (`self.Lerp Alpha`)))
  (`self.K2_SetActorLocation` _player_ref (+ (`KismetMathLibrary.Vector_SlerpNormals` (`KismetMathLibrary.Normal` (`self.Original Actor Location`)) (`KismetMathLibrary.Normal` (+ (`self.K2_GetActorLocation`) (* (`self.GetActorRightVector`) 100.0))) (`self.Lerp Alpha`)) (`self.K2_GetActorLocation` _player_ref)) false false))

(fn `UserConstructionScript`)
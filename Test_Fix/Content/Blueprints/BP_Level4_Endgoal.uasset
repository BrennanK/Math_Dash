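; BP_Level4_Endgoal is the end-of-level goal trigger for Level 4.
; When the player pawn overlaps its Box, it creates the end goal widget, adds it to the viewport and sets Game and UI input focused on it.
; It then freezes the game through zero global time dilation, hides the mouse cursor and plays the level-complete sound.
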(event `self.Box.OnComponentBeginOverlap`
  (params (OverlappedComponent :type "PrimitiveComponent Object Reference") (OtherActor :type "Actor Object Reference") (OtherComp :type "PrimitiveComponent Object Reference") (OtherBodyIndex :type Integer) (bFromSweep :type Boolean) (SweepResult :type "HitResult Structure (by ref)"))
  (if (== OtherActor (`GameplayStatics.GetPlayerPawn` 0))
    (`self.Create End Goal Widget`)))

(fn `Create End Goal Widget`
  (bind _returnvalue (`GameplayStatics.GetPlayerController` 0))
  (bind _returnvalue_2 (`|CreateWidget` "/Game/Widgets/BP_End_Goal_Widget.BP_End_Goal_Widget_C"))
  (`WidgetBlueprintLibrary.SetInputMode_GameAndUIEx` _returnvalue _returnvalue_2)
  (`UserWidget.AddToViewport` _returnvalue_2 0)
  (`GameplayStatics.SetGlobalTimeDilation` 0.0)
  (set `PlayerController.bShowMouseCursor` false _returnvalue)
  (`AudioComponent.Play` (`self.SFX_LevelComplete`) 0.0))

(fn `UserConstructionScript`)
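; Coin pickup actor that spins on a looping timer and adds to the player's coin count when touched by the third-person character.
; A sphere overlap with a box component on the character starts magnetization, a looping timer that steps the coin toward just below player pawn 0.
; Any other overlapping component of the character collects it, scaling the score by the powerup multiplier, updating the UI and destroying the coin.
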(event `self.ReceiveBeginPlay`
  (bind _returnvalue (`KismetSystemLibrary.K2_SetTimer` null "Rotate Coin" (/ 1.0 60.0) true))
  (set `self.Rotate Timer` _returnvalue))

(event `self.ReceiveTick`
  (params (DeltaSeconds :type "Float (single-precision)")))

(event `Rotate Coin`
  (bind (_returnvalue_roll _returnvalue_pitch _returnvalue_yaw) (`KismetMathLibrary.BreakRotator` (`self.K2_GetActorRotation`)))
  (`self.K2_SetActorRotation` (`KismetMathLibrary.MakeRotator` _returnvalue_roll _returnvalue_pitch (+ _returnvalue_yaw 1.0))))

(event `self.sphere.OnComponentBeginOverlap`
  (params (OverlappedComponent :type "PrimitiveComponent Object Reference") (OtherActor :type "Actor Object Reference") (OtherComp :type "PrimitiveComponent Object Reference") (OtherBodyIndex :type Integer) (bFromSweep :type Boolean) (SweepResult :type "HitResult Structure (by ref)"))
  (bind _asbp_third_person_character (cast `/Game/ThirdPerson/Blueprints/BP_ThirdPersonCharacter` OtherActor))
  (if (== (`GameplayStatics.GetObjectClass` OtherComp) "/Script/Engine.BoxComponent")
    (`self.Start Magnetization`)
    (else
      (bind _output_get (set `self.Coin score` (* (`self.Coin score`) (`/Game/ThirdPerson/Blueprints/Powerup_Component.Coin Mutiplier` (`/Game/ThirdPerson/Blueprints/BP_ThirdPersonCharacter.Powerup_Component` _asbp_third_person_character)))))
      (`/Game/Characters/Player_UI/W_MainPlayer.Update coin count` (`/Game/ThirdPerson/Blueprints/BP_ThirdPersonCharacter.Player UI Ref` _asbp_third_person_character) _output_get)
      (`KismetSystemLibrary.K2_ClearAndInvalidateTimerHandle` (`self.Rotate Timer`))
      (`self.K2_DestroyActor`))))

(event `Start Magnetization`
  (bind _returnvalue (`KismetSystemLibrary.K2_SetTimerDelegate` (delegate `Move toward Player`) (`GameplayStatics.GetWorldDeltaSeconds`) true))
  (set `self.Move Timer` _returnvalue))

(event `Move toward Player`
  (`self.K2_SetActorLocation` (+ (`self.K2_GetActorLocation`) (* (`KismetMathLibrary.Normal` (- (- (`self.K2_GetActorLocation` (`GameplayStatics.GetPlayerPawn` 0)) (0.0 0.0 20.0)) (`self.K2_GetActorLocation`))) (`self.Coin Lerp Speed`)))))

(fn `UserConstructionScript`)
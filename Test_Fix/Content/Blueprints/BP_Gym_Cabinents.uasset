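; BP_Gym_Cabinents is a gym cabinet prop that varies its look and makes a big-hit sound when the player character runs into it.
; On BeginPlay it sets CabinetMesh to a random entry from MeshArray.
; A Box overlap from BP_ThirdPersonCharacter plays the SFXBigHit2 audio from the start at full volume, with no guard against retriggering.
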(event `self.ReceiveBeginPlay`
  (bind _mesh_array (`self.Mesh Array`))
  (`StaticMeshComponent.SetStaticMesh` (`self.Cabinet mesh`) (`|GetArrayItem` _mesh_array (`KismetMathLibrary.RandomIntegerInRange` 0 (- (`KismetArrayLibrary.Array_Length` _mesh_array) 1)))))

(event `self.Box.OnComponentBeginOverlap`
  (params (OverlappedComponent :type "PrimitiveComponent Object Reference") (OtherActor :type "Actor Object Reference") (OtherComp :type "PrimitiveComponent Object Reference") (OtherBodyIndex :type Integer) (bFromSweep :type Boolean) (SweepResult :type "HitResult Structure (by ref)"))
  (bind _sfx_bighit_2 (`self.SFX_BigHit_2`))
  (cast `/Game/ThirdPerson/Blueprints/BP_ThirdPersonCharacter` OtherActor)
  (`AudioComponent.SetVolumeMultiplier` _sfx_bighit_2 1.0)
  (`AudioComponent.Play` _sfx_bighit_2 0.0))

(fn `UserConstructionScript`)
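; Blueprint that generates a random addition, subtraction, multiplication or division problem with one correct and three wrong answers.
; GenerateMathProblem sets per-operation answer ranges and derives operands so results are whole numbers, then debug-prints the answers.
; Recursive WrongAnswerGenerator screens against the never-cleared AlreadyGenerated set, but re-rolls on return and drops the recursive result.
; ReturnProblemComponents outputs operands, operation and answers.
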(event `Generate Math Problem`
  (bind _returnvalue (`KismetMathLibrary.RandomIntegerInRange` 1 10))
  (bind _already_generated (`self.Already Generated`))
  (bind _already_generated_2 (`self.Already Generated`))
  (bind _already_generated_3 (`self.Already Generated`))
  (switch `/Game/Blueprints/Operations` (cast `/Game/Blueprints/Operations` (`KismetMathLibrary.Conv_IntToByte` (`KismetMathLibrary.RandomIntegerInRange` 0 3))) ; 0
    (:`NewEnumerator0`
      (`|ExecutionSequence`
        (:`then_0`
          (set `self.Operations` "NewEnumerator0"))
        (:`then_1`
          (bind _output_get (set `self.AnsRangeLow` 2)))
        (:`then_2`
          (bind _output_get_2 (set `self.AnsRangeHigh` 99)))
        (:`then_3`
          (bind _output_get_3 (set `self.ans_correct` (`KismetMathLibrary.RandomIntegerInRange` _output_get _output_get_2)))
          (bind _output_get_4 (set `self.Var_1` (`KismetMathLibrary.RandomIntegerInRange` 1 _output_get_3)))
          (set `self.Var_2` (- _output_get_3 _output_get_4))
          (`KismetSystemLibrary.PrintString` null (`KismetStringLibrary.Conv_IntToString` (`self.ans_correct`)) true true (struct :`R` 1.0 :`G` 0.834536 :`A` 1.0) 120.0 :!label _label)
          (`BlueprintSetLibrary.Set_Add` _already_generated (`self.ans_correct`))
          (bind _wronganswer (`self.WrongAnswerGenerator` (`self.AnsRangeLow`) (`self.AnsRangeHigh`) _already_generated))
          (`BlueprintSetLibrary.Set_Add` _already_generated_2 _wronganswer)
          (set `self.ans_wrong_1` _wronganswer)
          (bind _wronganswer_2 (`self.WrongAnswerGenerator` (`self.AnsRangeLow`) (`self.AnsRangeHigh`) _already_generated_2))
          (`BlueprintSetLibrary.Set_Add` _already_generated_3 _wronganswer_2)
          (set `self.ans_wrong_2` _wronganswer_2)
          (bind _wronganswer_3 (`self.WrongAnswerGenerator` (`self.AnsRangeLow`) (`self.AnsRangeHigh`) _already_generated_3))
          (`BlueprintSetLibrary.Set_Add` (`self.Already Generated`) _wronganswer_3)
          (set `self.ans_wrong_3` _wronganswer_3)
          (bind _result (`BlueprintSetLibrary.Set_ToArray` (`self.Already Generated`)))
          (for _array_element _result
            (`KismetSystemLibrary.PrintString` null (`KismetStringLibrary.Conv_IntToString` _array_element) true true (struct :`R` 0.779226 :`G` 0.034167 :`B` 1.0 :`A` 1.0) 120.0)))))
    (:`NewEnumerator1`
      (`|ExecutionSequence`
        (:`then_0`
          (set `self.Operations` "NewEnumerator1"))
        (:`then_1`
          (bind _output_get_5 (set `self.AnsRangeLow` 1)))
        (:`then_2`
          (bind _output_get_6 (set `self.AnsRangeHigh` 15)))
        (:`then_3`
          (bind _output_get_7 (set `self.ans_correct` (`KismetMathLibrary.RandomIntegerInRange` _output_get_5 _output_get_6)))
          (bind _output_get_8 (set `self.Var_2` (`KismetMathLibrary.RandomIntegerInRange` (`self.AnsRangeLow`) (- 100 (`self.AnsRangeHigh`)))))
          (set `self.Var_1` (+ _output_get_7 _output_get_8))
          (goto _label))))
    (:`NewEnumerator2`
      (`|ExecutionSequence`
        (:`then_0`
          (set `self.Operations` "NewEnumerator2"))
        (:`then_1`
          (set `self.AnsRangeLow` 1))
        (:`then_2`
          (set `self.AnsRangeHigh` 100))
        (:`then_3`
          (bind _output_get_9 (set `self.Var_1` _returnvalue))
          (bind _output_get_10 (set `self.Var_2` _returnvalue))
          (set `self.ans_correct` (* _output_get_9 _output_get_10))
          (goto _label))))
    (:`NewEnumerator3`
      (`|ExecutionSequence`
        (:`then_0`
          (set `self.Operations` "NewEnumerator3"))
        (:`then_1`
          (bind _output_get_11 (set `self.AnsRangeLow` 2)))
        (:`then_2`
          (bind _output_get_12 (set `self.AnsRangeHigh` 10)))
        (:`then_3`
          (bind _output_get_13 (set `self.ans_correct` (`KismetMathLibrary.RandomIntegerInRange` _output_get_11 _output_get_12)))
          (bind _output_get_14 (set `self.Var_2` (`KismetMathLibrary.RandomIntegerInRange` _output_get_11 _output_get_12)))
          (set `self.Var_1` (* _output_get_13 _output_get_14))
          (goto _label))))))

(fn `Return Problem Components`
  (returns (var1_out :type Integer) (var2_out :type Integer) (correct_out :type Integer) (wrong1_out :type Integer) (wrong2_out :type Integer) (wrong3_out :type Integer) (op_out :type "/Game/Blueprints/Operations Enum"))
  (return (`self.Var_1`) (`self.Var_2`) (`self.ans_correct`) (`self.ans_wrong_1`) (`self.ans_wrong_2`) (`self.ans_wrong_3`) (`self.Operations`)))

(fn `WrongAnswerGenerator`
  (params (LowerBound :type Integer) (UpperBound :type Integer) (Exclude :type "Set of Integer"))
  (returns (WrongAnswer :type Integer))
  (bind _returnvalue (`KismetMathLibrary.RandomIntegerInRange` LowerBound UpperBound))
  (if (`BlueprintSetLibrary.Set_Contains` Exclude _returnvalue)
    (`self.WrongAnswerGenerator` LowerBound UpperBound Exclude)
    (else
      (return _returnvalue))))
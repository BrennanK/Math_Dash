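; BP_Cross_Section is a procedurally chained school hallway segment with obstacles, coins and math-problem triggers.
; BeginPlay randomly picks forward, left or right, adjusts branch geometry, randomizes lockers and math triggers, and spawns hazards and coins at placeholder components.
; Player overlap with ForwardSpawnBox spawns the next segment at the chosen exit and registers it with BP_ProceduralBuilder, or spawns an end goal when flagged.
; BP_Teacher overlapping the entry has the builder remove the segment.
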(event `Wet floor spawn`
  (for _array_element (`|MakeArray` (`self.Wet floor`) (`self.Wet floor1`) (`self.Wet floor2`) (`self.Wet floor3`) (`self.Wet floor4`) (`self.Wet floor5`))
    (`|SpawnActorFromClass` "/Game/Blueprints/BP_Wet_Floor_Sign.BP_Wet_Floor_Sign_C" (`KismetMathLibrary.MakeTransform` (`SceneComponent.K2_GetComponentLocation` _array_element) (`SceneComponent.K2_GetComponentRotation` _array_element) (1.5 1.5 1.5)) "Undefined" "MultiplyWithRoot" null null)
    (`SceneComponent.SetVisibility` _array_element false false)
    (`PrimitiveComponent.SetCollisionEnabled` _array_element "NoCollision")))

(event `Backpack spawn`
  (bind _array (`|MakeArray` (`self.Backpack1`) (`self.Backpack2`) (`self.Backpack3`) (`self.Backpack4`) (`self.Backpack5`) (`self.Backpack6`) (`self.Backpack7`) (`self.Backpack`) (`self.Backpack8`) (`self.Backpack9`) (`self.Backpack10`) (`self.Backpack11`) (`self.Backpack12`)))
  (`|ExecutionSequence`
    (:`then_0`
      (for _array_element _array
        (`SceneComponent.SetVisibility` _array_element (`KismetMathLibrary.RandomBool`) false)))
    (:`then_1`
      (for _array_element_2 _array
        (if (`SceneComponent.bVisible` _array_element_2)
          (`|SpawnActorFromClass` "/Game/Blueprints/BP_Backpack.BP_Backpack_C" (`KismetMathLibrary.MakeTransform` (`SceneComponent.K2_GetComponentLocation` _array_element_2) (struct) (0.5 0.5 0.5)) "Undefined" "MultiplyWithRoot" null null)
          (`SceneComponent.SetVisibility` _array_element_2 false false)
          (`PrimitiveComponent.SetCollisionEnabled` _array_element_2 "NoCollision"))))))

(event `Random coin spawn`
  (switch `/Game/Blueprints/Turn_Directions` (`self.Turn directions ref`)
    (:`NewEnumerator0`
      (`self.Left floor coins spawn`))
    (:`NewEnumerator1`
      (`self.Right floor coins spawn`))
    (:`NewEnumerator2`
      (`self.Forward Coins spawn`))))

(event `Right floor coins spawn`
  (for _array_element (`|MakeArray` (`self.Right floor coins4`))
    (bind _returnvalue (`SceneComponent.K2_GetComponentToWorld` _array_element))
    (bind _returnvalue_2 (`|SpawnActorFromClass` "/Game/Blueprints/CoinBP.CoinBP_C" (`KismetMathLibrary.MakeTransform` (`KismetMathLibrary.MakeVector` (.x (.location _returnvalue)) (.y (.location _returnvalue)) (.z (.location _returnvalue))) (.rotation _returnvalue)) "AdjustIfPossibleButAlwaysSpawn" "MultiplyWithRoot" null null))
    (`self.Coin instance` _returnvalue_2 (`KismetMathLibrary.RandomIntegerInRange` 1 7) 100.0)))

(event `Locker collision check`
  (`|ExecutionSequence`
    (:`then_0`
      (for _array_element (`|MakeArray` (`self.Lockers 7`) (`self.Lockers 6`) (`self.Lockers 5`) (`self.Lockers 8`) (`self.Lockers 4`) (`self.Lockers 9`) (`self.Lockers 10`) (`self.Lockers 11`) (`self.Lockers 12`) (`self.Lockers 13`) (`self.Lockers 15`) (`self.Lockers 16`) (`self.Lockers 17`) (`self.Lockers 18`) (`self.Lockers 19`) (`self.Lockers 23`) (`self.Lockers 27`) (`self.Lockers 31`) (`self.Lockers 34`) (`self.Lockers 38`) (`self.Lockers 39`) (`self.Lockers 40`) (`self.Lockers 44`) (`self.Lockers 45`) (`self.Lockers 47`) (`self.Lockers 49`) (`self.Lockers 51`) (`self.Lockers 52`) (`self.Lockers 53`) (`self.Lockers 54`) (`self.Lockers 56`) (`self.Lockers 57`) (`self.Lockers 58`) (`self.Lockers 59`) (`self.Lockers 62`))
        (`SceneComponent.SetVisibility` _array_element (`KismetMathLibrary.RandomBool`) false)))
    (:`then_1`
      (for _array_element_2 (`|MakeArray` (`self.Lockers 7`) (`self.Lockers 6`) (`self.Lockers 5`) (`self.Lockers 8`) (`self.Lockers 4`) (`self.Lockers 9`) (`self.Lockers 10`) (`self.Lockers 11`) (`self.Lockers 12`) (`self.Lockers 13`) (`self.Lockers 15`) (`self.Lockers 16`) (`self.Lockers 17`) (`self.Lockers 18`) (`self.Lockers 19`) (`self.Lockers 23`) (`self.Lockers 27`) (`self.Lockers 31`) (`self.Lockers 34`) (`self.Lockers 38`) (`self.Lockers 39`) (`self.Lockers 40`) (`self.Lockers 44`) (`self.Lockers 45`) (`self.Lockers 47`) (`self.Lockers 49`) (`self.Lockers 51`) (`self.Lockers 52`) (`self.Lockers 53`) (`self.Lockers 54`) (`self.Lockers 56`) (`self.Lockers 57`) (`self.Lockers 58`) (`self.Lockers 59`) (`self.Lockers 62`))
        (if (`SceneComponent.bVisible` _array_element_2)
          (`PrimitiveComponent.SetCollisionEnabled` _array_element_2 "QueryAndPhysics")
          (else
            (`PrimitiveComponent.SetCollisionEnabled` _array_element_2 "NoCollision")))))))

(event `Left floor coins spawn`
  (for _array_element (`|MakeArray` (`self.Left segement coin`))
    (while false
      (bind _returnvalue (`SceneComponent.K2_GetComponentToWorld` _array_element))
      (bind _returnvalue_2 (`|SpawnActorFromClass` "/Game/Blueprints/CoinBP.CoinBP_C" (`KismetMathLibrary.MakeTransform` (`KismetMathLibrary.MakeVector` (.x (.location _returnvalue)) 0.0 (.z (.location _returnvalue))) (.rotation _returnvalue)) "AdjustIfPossibleButAlwaysSpawn" "MultiplyWithRoot" null null))
      (`self.Coin instance` _returnvalue_2 (`KismetMathLibrary.RandomIntegerInRange` 1 7) 100.0))))

(event `Forward Coins spawn`
  (for _array_element (`|MakeArray` (`self.Forward coins2`))
    (bind _returnvalue (`SceneComponent.K2_GetComponentToWorld` _array_element))
    (bind _returnvalue_2 (`|SpawnActorFromClass` "/Game/Blueprints/CoinBP.CoinBP_C" (`KismetMathLibrary.MakeTransform` (`KismetMathLibrary.MakeVector` (.x (.location _returnvalue)) (.y (.location _returnvalue)) (.z (.location _returnvalue))) (.rotation _returnvalue)) "AdjustIfPossibleButAlwaysSpawn" "MultiplyWithRoot" null null))
    (`self.Coin instance` _returnvalue_2 (`KismetMathLibrary.RandomIntegerInRange` 1 7) 100.0)))

(event `self.ReceiveBeginPlay`
  (`|ExecutionSequence`
    (:`then_0`
      (bind _outactors (`GameplayStatics.GetAllActorsOfClass` "/Game/ThirdPerson/Blueprints/BP_ThirdPersonCharacter.BP_ThirdPersonCharacter_C"))
      (set `self.PlayerRef` (`|GetArrayItem` _outactors))
      (bind _output_get (set `PrimitiveComponent.bGenerateOverlapEvents` (`KismetMathLibrary.RandomBool`) (`self.Turn box`)))
      (if (== _output_get false)
        (`self.Set up Forward Direction`)
        (else
          (`self.Setup Turn Direction`))))
    (:`then_1`
      (set `PrimitiveComponent.bGenerateOverlapEvents` (`KismetMathLibrary.RandomBool`) (`self.Left Segment Left side Math Problem Box collision`))
      (set `PrimitiveComponent.bGenerateOverlapEvents` (`KismetMathLibrary.RandomBool`) (`self.Forward  Math Problem Box collision`))
      (set `PrimitiveComponent.bGenerateOverlapEvents` (`KismetMathLibrary.RandomBool`) (`self.Right Segment Right side Math Problem Box collision`)))
    (:`then_2`
      (`self.Locker collision check`)
      (`self.Glue spill spawn`)
      (`self.Fallen lockers spawn`)
      (`self.shattered papers spawn`)
      (`self.Wet floor spawn`)
      (`self.Random coin spawn`))))

(event `Random left side wall`
  (switch `int` (`KismetMathLibrary.RandomIntegerInRange` 0 4)))

(event `self.Turn box.OnComponentBeginOverlap`
  (params (OverlappedComponent :type "PrimitiveComponent Object Reference") (OtherActor :type "Actor Object Reference") (OtherComp :type "PrimitiveComponent Object Reference") (OtherBodyIndex :type Integer) (bFromSweep :type Boolean) (SweepResult :type "HitResult Structure (by ref)"))
  (cast `/Game/ThirdPerson/Blueprints/BP_ThirdPersonCharacter` OtherActor))

(event `self.Left Segment Left side Math Problem Box collision.OnComponentBeginOverlap`
  (params (OverlappedComponent :type "PrimitiveComponent Object Reference") (OtherActor :type "Actor Object Reference") (OtherComp :type "PrimitiveComponent Object Reference") (OtherBodyIndex :type Integer) (bFromSweep :type Boolean) (SweepResult :type "HitResult Structure (by ref)"))
  ;[1 1 1] Spawns a Math Problem on the Left Side
  (cast `/Game/ThirdPerson/Blueprints/BP_ThirdPersonCharacter` OtherActor)
  (`|SpawnActorFromClass` "/Game/Blueprints/MathProblem_UI.MathProblem_UI_C" (`SceneComponent.K2_GetComponentToWorld` (`self.Left Segment Left side Math Problem Box collision`)) "Undefined" "MultiplyWithRoot" null null))

(event `self.Forward spawn box.OnComponentBeginOverlap`
  (params (OverlappedComponent :type "PrimitiveComponent Object Reference") (OtherActor :type "Actor Object Reference") (OtherComp :type "PrimitiveComponent Object Reference") (OtherBodyIndex :type Integer) (bFromSweep :type Boolean) (SweepResult :type "HitResult Structure (by ref)"))
  ;[1 1 1] Procedural Generated Event for Cross Section
  (cast `/Game/ThirdPerson/Blueprints/BP_ThirdPersonCharacter` OtherActor)
  (switch `/Game/Blueprints/Turn_Directions` (`self.Turn directions ref`)
    (:`NewEnumerator0`
      (`self.Spawn Cross section at the Left End`))
    (:`NewEnumerator1`
      (`self.Spawn Cross Section at Right End`))
    (:`NewEnumerator2`
      (`self.Spawn Cross Section at the Forward end`))))

(event `self.Forward  Math Problem Box collision.OnComponentBeginOverlap`
  (params (OverlappedComponent :type "PrimitiveComponent Object Reference") (OtherActor :type "Actor Object Reference") (OtherComp :type "PrimitiveComponent Object Reference") (OtherBodyIndex :type Integer) (bFromSweep :type Boolean) (SweepResult :type "HitResult Structure (by ref)"))
  ;[1 1 1] Spawn A
  (cast `/Game/ThirdPerson/Blueprints/BP_ThirdPersonCharacter` OtherActor)
  (`|SpawnActorFromClass` "/Game/Blueprints/MathProblem_UI.MathProblem_UI_C" (`SceneComponent.K2_GetComponentToWorld` (`self.Forward  Math Problem Box collision`)) "Undefined" "MultiplyWithRoot" null null))

(event `self.Right Segment Right side Math Problem Box collision.OnComponentBeginOverlap`
  (params (OverlappedComponent :type "PrimitiveComponent Object Reference") (OtherActor :type "Actor Object Reference") (OtherComp :type "PrimitiveComponent Object Reference") (OtherBodyIndex :type Integer) (bFromSweep :type Boolean) (SweepResult :type "HitResult Structure (by ref)"))
  (cast `/Game/ThirdPerson/Blueprints/BP_ThirdPersonCharacter` OtherActor)
  (`|SpawnActorFromClass` "/Game/Blueprints/MathProblem_UI.MathProblem_UI_C" (`SceneComponent.K2_GetComponentToWorld` (`self.Right Segment Right side Math Problem Box collision`)) "Undefined" "MultiplyWithRoot" null null))

(event `self.Entry Destroy actor collision.OnComponentBeginOverlap`
  (params (OverlappedComponent :type "PrimitiveComponent Object Reference") (OtherActor :type "Actor Object Reference") (OtherComp :type "PrimitiveComponent Object Reference") (OtherBodyIndex :type Integer) (bFromSweep :type Boolean) (SweepResult :type "HitResult Structure (by ref)"))
  ;[1 1 1] This destoys the actor
  (cast `/Game/Blueprints/BP_Teacher` OtherActor)
  (`/Game/Blueprints/BP_ProceduralBuilder.Remove segment` (`self.Builder REF`) self))

(event `Find Builder`
  (bind _outactors (`GameplayStatics.GetAllActorsOfClass` "/Game/Blueprints/BP_ProceduralBuilder.BP_ProceduralBuilder_C"))
  (set `self.Builder REF` (`|GetArrayItem` _outactors)))

(event `Glue spill spawn`
  (`/Engine/EditorBlueprintResources/StandardMacros.DoOnce` false
    (:`Completed`
      (for _array_element (`|MakeArray` (`self.Entry Glue spill scene`) (`self.Entry Glue spill scene 2`) (`self.Entry floor spill scene 1`) (`self.Right floor Glue spill scene 3`) (`self.Right Glue spill scene 4`) (`self.Right floor Glue spill scene5`) (`self.forward Glue spill scene6`) (`self.forward Glue spill scene7`) (`self.Left Glue spill scene9`) (`self.left Glue spill scene10`) (`self.left Glue spill scene11`) (`self.forward Glue spill scene8`))
        (`|SpawnActorFromClass` "/Game/Blueprints/BP_Glue_Spill.BP_Glue_Spill_C" (`KismetMathLibrary.MakeTransform` (`SceneComponent.K2_GetComponentLocation` _array_element)) "AdjustIfPossibleButAlwaysSpawn" "MultiplyWithRoot" null null)))))

(event `Fallen lockers spawn`
  (bind (_returnvalue_roll _returnvalue_pitch _returnvalue_yaw) (`KismetMathLibrary.BreakRotator` (`KismetMathLibrary.MakeRotator` 0.0)))
  (bind _returnvalue (`KismetMathLibrary.RandomFloatInRange` _returnvalue_yaw 45.0))
  (for (_array_element _array_index) (`|MakeArray` (`self.Fallen lockers scene`) (`self.Fallen lockers scene1`) (`self.Fallen lockers scene2`) (`self.Fallen lockers scene3`) (`self.Fallen lockers scene4`) (`self.Fallen lockers scene5`) (`self.Fallen lockers scene6`) (`self.Fallen lockers scene7`) (`self.Fallen lockers scene8`))
    (switch `int` _array_index
      (:`0`
        (`|SpawnActorFromClass` "/Game/Blueprints/BP_Open_Fallen_Locker1.BP_Open_Fallen_Locker1_C" (`KismetMathLibrary.MakeTransform` (`SceneComponent.K2_GetComponentLocation` _array_element) (`KismetMathLibrary.MakeRotator` 0.0 0.0 _returnvalue)) "AdjustIfPossibleButAlwaysSpawn" "MultiplyWithRoot" null null :!label _label))
      (:`1`
        (`|SpawnActorFromClass` "/Game/Blueprints/BP_Open_Fallen_Locker2.BP_Open_Fallen_Locker2_C" (`KismetMathLibrary.MakeTransform` (`SceneComponent.K2_GetComponentLocation` _array_element) (`KismetMathLibrary.MakeRotator` 0.0 0.0 _returnvalue)) "AdjustIfPossibleButAlwaysSpawn" "MultiplyWithRoot" null null :!label _label_2))
      (:`2`
        (`|SpawnActorFromClass` "/Game/Blueprints/BP_Open_Fallen_Locker3.BP_Open_Fallen_Locker3_C" (`KismetMathLibrary.MakeTransform` (`SceneComponent.K2_GetComponentLocation` _array_element) (`KismetMathLibrary.MakeRotator` 0.0 0.0 _returnvalue)) "AdjustIfPossibleButAlwaysSpawn" "MultiplyWithRoot" null null :!label _label_3))
      (:`3`
        (goto _label))
      (:`4`
        (goto _label_2))
      (:`5`
        (goto _label_3))
      (:`6`
        (goto _label))
      (:`7`
        (goto _label_2))
      (:`8`
        (goto _label_3)))))

(event `shattered papers spawn`
  (for _array_element (`|MakeArray` (`self.Shattered pages screen1`) (`self.Shattered pages screen`) (`self.Shattered pages screen2`) (`self.Shattered pages screen3`) (`self.Shattered pages screen4`) (`self.Shattered pages screen5`) (`self.Shattered pages screen6`) (`self.Shattered pages screen7`))
    (`|SpawnActorFromClass` "/Game/Blueprints/BP_Scattered_Pages.BP_Scattered_Pages_C" (`KismetMathLibrary.MakeTransform` (`SceneComponent.K2_GetComponentLocation` _array_element)) "Undefined" "MultiplyWithRoot" null null)))

(fn `Calculate Forward location and Rotation`
  (returns (ReturnValue :type "Vector Structure") (ReturnValue2 :type "Rotator Structure"))
  (return (+ (`SceneComponent.K2_GetComponentLocation` (`self.Forward floor`)) (* (`self.GetActorForwardVector`) (`self.Gap value`))) (`self.K2_GetActorRotation`)))

(fn `Calculate Left Location and Rotation`
  (returns (ReturnValue :type "Vector Structure") (ReturnValue_Roll :type "Float (single-precision)") (ReturnValue_Pitch :type "Float (single-precision)") (ReturnValue2 :type "Float (double-precision)"))
  (bind (_returnvalue_roll _returnvalue_pitch _returnvalue_yaw) (`KismetMathLibrary.BreakRotator` (`self.K2_GetActorRotation`)))
  (return (+ (`SceneComponent.K2_GetComponentLocation` (`self.Left Segment Leftfloor`)) (* (* (`self.GetActorRightVector`) -1.0) (`self.Gap value`))) _returnvalue_roll _returnvalue_pitch (- _returnvalue_yaw 90.0)))

(fn `Calculate Right Location and Rotation`
  (returns (ReturnValue :type "Vector Structure") (ReturnValue_Roll :type "Float (single-precision)") (ReturnValue_Pitch :type "Float (single-precision)") (ReturnValue2 :type "Float (double-precision)"))
  (bind (_returnvalue_roll _returnvalue_pitch _returnvalue_yaw) (`KismetMathLibrary.BreakRotator` (`self.K2_GetActorRotation`)))
  (return (+ (`SceneComponent.K2_GetComponentLocation` (`self.Right Segment Right Floor`)) (* (`self.GetActorRightVector`) (`self.Gap value`))) _returnvalue_roll _returnvalue_pitch (+ _returnvalue_yaw 90.0)))

(fn `Coin instance`
  (params (`Coin REF` :type "/Game/Blueprints/CoinBP Object Reference") (`number of coins ` :type Integer :default 0) (`space between coins` :type "Float (double-precision)" :default 200.0))
  (bind (_returnvalue_location _returnvalue_rotation _returnvalue_scale) (`KismetMathLibrary.BreakTransform` (`self.GetTransform` `Coin REF`)))
  (for _index (range 1 (+ `number of coins ` 1))
    (`|SpawnActorFromClass` (`GameplayStatics.GetObjectClass` `Coin REF`) (`KismetMathLibrary.MakeTransform` (+ _returnvalue_location (* (`self.GetActorForwardVector` `Coin REF`) `space between coins` _index)) _returnvalue_rotation _returnvalue_scale) "Undefined" "MultiplyWithRoot" null null)))

(fn `Set up Forward Direction`
  (bind _left_segment_leftfloor (`self.Left Segment Leftfloor`))
  (bind _left_segment_right_wall_right_side (`self.Left Segment Right Wall Right side`))
  (bind _left_segment_leftwall_left_side (`self.Left Segment Leftwall left side`))
  (bind _right_segment_right_floor (`self.Right Segment Right Floor`))
  (bind _right_segment_rightfllor_right_side (`self.Right Segment Rightfllor Right Side`))
  (bind _right_segment__left_wall_left_side (`self.Right Segment  Left wall left side`))
  (`SceneComponent.SetVisibility` (`self.Forward connector`) true false)
  (`|ExecutionSequence`
    (:`then_0`
      (`|ExecutionSequence`
        (:`then_0`
          (`SceneComponent.SetVisibility` _left_segment_leftfloor false false)
          (`SceneComponent.SetVisibility` _left_segment_right_wall_right_side false false)
          (`SceneComponent.SetVisibility` _left_segment_leftwall_left_side false false))
        (:`then_1`
          (`PrimitiveComponent.SetCollisionEnabled` _left_segment_leftfloor "NoCollision")
          (`PrimitiveComponent.SetCollisionEnabled` _left_segment_right_wall_right_side "NoCollision")
          (`PrimitiveComponent.SetCollisionEnabled` _left_segment_leftwall_left_side "QueryAndPhysics"))))
    (:`then_1`
      (`|ExecutionSequence`
        (:`then_0`
          (`SceneComponent.SetVisibility` _right_segment_right_floor false false)
          (`SceneComponent.SetVisibility` _right_segment_rightfllor_right_side false false)
          (`SceneComponent.SetVisibility` _right_segment__left_wall_left_side false false))
        (:`then_1`
          (`PrimitiveComponent.SetCollisionEnabled` _right_segment_right_floor "QueryAndPhysics")
          (`PrimitiveComponent.SetCollisionEnabled` _right_segment_rightfllor_right_side "QueryAndPhysics")
          (`PrimitiveComponent.SetCollisionEnabled` _right_segment__left_wall_left_side "QueryAndPhysics"))))
    (:`then_2`
      (set `self.Turn directions ref` "NewEnumerator2"))))

(fn `Setup Turn Direction`
  (bind _left_segment_leftfloor (`self.Left Segment Leftfloor`))
  (bind _left_segment_right_wall_right_side (`self.Left Segment Right Wall Right side`))
  (bind _left_segment_leftwall_left_side (`self.Left Segment Leftwall left side`))
  (bind _right_segment_right_floor (`self.Right Segment Right Floor`))
  (bind _right_segment_rightfllor_right_side (`self.Right Segment Rightfllor Right Side`))
  (bind _right_segment__left_wall_left_side (`self.Right Segment  Left wall left side`))
  (bind _left_connector (`self.Left connector`))
  (bind _right_connector (`self.right connector`))
  (bind _returnvalue (`|SpawnActorFromClass` "/Game/Blueprints/Turn_Collision.Turn_Collision_C" (`SceneComponent.K2_GetComponentToWorld` (`self.Turn box`)) "Undefined" "MultiplyWithRoot" null null))
  (switch `int` (`KismetMathLibrary.RandomIntegerInRange` (`self.Random integer`) 1)
    (:`0`
      (set `/Game/Blueprints/Turn_Collision.Left Or Right` "NewEnumerator1" _returnvalue)
      (`|ExecutionSequence`
        (:`then_0`
          (`SceneComponent.SetVisibility` _left_segment_leftfloor false false)
          (`SceneComponent.SetVisibility` _left_segment_right_wall_right_side false false)
          (`SceneComponent.SetVisibility` _left_segment_leftwall_left_side false false)
          (`SceneComponent.SetVisibility` _right_connector true false))
        (:`then_1`
          (`PrimitiveComponent.SetCollisionEnabled` _left_segment_leftfloor "NoCollision")
          (`PrimitiveComponent.SetCollisionEnabled` _left_segment_right_wall_right_side "NoCollision")
          (`PrimitiveComponent.SetCollisionEnabled` _left_segment_leftwall_left_side "NoCollision")
          (`PrimitiveComponent.SetCollisionEnabled` _right_connector "NoCollision"))
        (:`then_2`
          (set `self.Turn directions ref` "NewEnumerator1"))))
    (:`1`
      (set `/Game/Blueprints/Turn_Collision.Left Or Right` "NewEnumerator0" _returnvalue)
      (`|ExecutionSequence`
        (:`then_0`
          (`SceneComponent.SetVisibility` _right_segment_right_floor false false)
          (`SceneComponent.SetVisibility` _right_segment_rightfllor_right_side false false)
          (`SceneComponent.SetVisibility` _right_segment__left_wall_left_side false false)
          (`SceneComponent.SetVisibility` _left_connector true false))
        (:`then_1`
          (`PrimitiveComponent.SetCollisionEnabled` _right_segment_right_floor "NoCollision")
          (`PrimitiveComponent.SetCollisionEnabled` _right_segment_rightfllor_right_side "NoCollision")
          (`PrimitiveComponent.SetCollisionEnabled` _right_segment__left_wall_left_side "NoCollision")
          (`PrimitiveComponent.SetCollisionEnabled` _left_connector "NoCollision"))
        (:`then_2`
          (set `self.Turn directions ref` "NewEnumerator0"))))))

(fn `Spawn Cross Section at Right End`
  (if (`/Game/Blueprints/BP_ProceduralBuilder.SpawnEndGoal?` (`self.Builder REF`))
    (set `self.Gap value` 1650.0)
    (bind (_returnvalue _returnvalue_roll _returnvalue_pitch _returnvalue2) (`self.Calculate Right Location and Rotation`))
    (`|SpawnActorFromClass` "/Game/Blueprints/BP_Spawn_Endgoal.BP_Spawn_Endgoal_C" (`KismetMathLibrary.MakeTransform` _returnvalue (`KismetMathLibrary.MakeRotator` _returnvalue_roll _returnvalue_pitch _returnvalue2)) "Undefined" "MultiplyWithRoot" null null)
    (else
      (bind (_returnvalue_2 _returnvalue_roll_2 _returnvalue_pitch_2 _returnvalue2_2) (`self.Calculate Right Location and Rotation`))
      (bind _returnvalue_3 (`|SpawnActorFromClass` "BP_Cross_Section_C" (`KismetMathLibrary.MakeTransform` _returnvalue_2 (`KismetMathLibrary.MakeRotator` _returnvalue_roll_2 _returnvalue_pitch_2 _returnvalue2_2)) "Undefined" "MultiplyWithRoot" null null))
      (`/Game/Blueprints/BP_ProceduralBuilder.Add to Segments` (`self.Builder REF`) _returnvalue_3))))

(fn `Spawn Cross Section at the Forward end`
  (if (`/Game/Blueprints/BP_ProceduralBuilder.SpawnEndGoal?` (`self.Builder REF`))
    (set `self.Gap value` 1650.0)
    (bind (_returnvalue _returnvalue2) (`self.Calculate Forward location and Rotation`))
    (`|SpawnActorFromClass` "/Game/Blueprints/BP_Spawn_Endgoal.BP_Spawn_Endgoal_C" (`KismetMathLibrary.MakeTransform` _returnvalue _returnvalue2) "Undefined" "MultiplyWithRoot" null null)
    (else
      (bind (_returnvalue_2 _returnvalue2_2) (`self.Calculate Forward location and Rotation`))
      (bind _returnvalue_3 (`|SpawnActorFromClass` "BP_Cross_Section_C" (`KismetMathLibrary.MakeTransform` _returnvalue_2 _returnvalue2_2) "Undefined" "MultiplyWithRoot" null null))
      (`/Game/Blueprints/BP_ProceduralBuilder.Add to Segments` (`self.Builder REF`) _returnvalue_3))))

(fn `Spawn Cross section at the Left End`
  (if (`/Game/Blueprints/BP_ProceduralBuilder.SpawnEndGoal?` (`self.Builder REF`))
    (set `self.Gap value` 1650.0)
    (bind (_returnvalue _returnvalue_roll _returnvalue_pitch _returnvalue2) (`self.Calculate Left Location and Rotation`))
    (`|SpawnActorFromClass` "/Game/Blueprints/BP_Spawn_Endgoal.BP_Spawn_Endgoal_C" (`KismetMathLibrary.MakeTransform` _returnvalue (`KismetMathLibrary.MakeRotator` _returnvalue_roll _returnvalue_pitch _returnvalue2)) "Undefined" "MultiplyWithRoot" null null)
    (else
      (bind (_returnvalue_2 _returnvalue_roll_2 _returnvalue_pitch_2 _returnvalue2_2) (`self.Calculate Left Location and Rotation`))
      (bind _returnvalue_3 (`|SpawnActorFromClass` "BP_Cross_Section_C" (`KismetMathLibrary.MakeTransform` _returnvalue_2 (`KismetMathLibrary.MakeRotator` _returnvalue_roll_2 _returnvalue_pitch_2 _returnvalue2_2)) "Undefined" "MultiplyWithRoot" null null))
      (`/Game/Blueprints/BP_ProceduralBuilder.Add to Segments` (`self.Builder REF`) _returnvalue_3))))

(fn `UserConstructionScript`)
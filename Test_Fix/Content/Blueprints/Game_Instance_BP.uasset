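; Game instance that loads persistent player data (coins, music volume and SFX volume) when the game initializes.
; On Init it checks Slot1 for a save and, if none exists, creates a BP_Save object and writes it to that slot.
; It then loads the slot, casts it to BP_Save and copies the saved wallet amount and both volume settings into its own variables.
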(event `self.ReceiveInit`
  (bind _returnvalue (`GameplayStatics.DoesSaveGameExist` "Slot1"))
  (if (not _returnvalue)
    (`GameplayStatics.CreateSaveGameObject` "/Game/Blueprints/BP_Save.BP_Save_C")
    (`GameplayStatics.SaveGameToSlot` null "Slot1"))
  (bind _returnvalue_2 (`GameplayStatics.LoadGameFromSlot` "Slot1"))
  (bind _asbp_save (cast `/Game/Blueprints/BP_Save` _returnvalue_2))
  (set `self.Coins` (`/Game/Blueprints/BP_Save.Wallet Amount` _asbp_save))
  (set `self.Music Volume` (`/Game/Blueprints/BP_Save.Music Volume Saved` _asbp_save))
  (set `self.SFX Volume` (`/Game/Blueprints/BP_Save.SFX Volume Saved` _asbp_save)))
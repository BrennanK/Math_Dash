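; BP_YogaMat is a yoga mat obstacle that slows the player who steps onto it.
; On BeginPlay it picks a random mesh from an array of mat variants for visual variety.
; When the player character overlaps its box, it calls the character's negative speed-change message with the configured slow amount and duration, then plays a sound.
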(event `self.ReceiveBeginPlay`
  (bind _yoga_mats (`self.Yoga MAts`))
  (`StaticMeshComponent.SetStaticMesh` (`self.Yoga Mat Mesh`) (`|GetArrayItem` _yoga_mats (`KismetMathLibrary.RandomIntegerInRange` 0 (- (`KismetArrayLibrary.Array_Length` _yoga_mats) 1)))))

(event `self.ReceiveActorBeginOverlap`
  (params (OtherActor :type "Actor Object Reference")))

(event `self.Box.OnComponentBeginOverlap`
  (params (OverlappedComponent :type "PrimitiveComponent Object Reference") (OtherActor :type "Actor Object Reference") (OtherComp :type "PrimitiveComponent Object Reference") (OtherBodyIndex :type Integer) (bFromSweep :type Boolean) (SweepResult :type "HitResult Structure (by ref)"))
  (bind _returnvalue (`GameplayStatics.GetPlayerCharacter` 0))
  (bind _audio (`self.Audio`))
  (if (== OtherActor _returnvalue)
    (message `/Game/Blueprints/BPI_PlayerCharacter.Set Speed Diff and Duration Negative` _returnvalue (`self.Slow`) (`self.Duration`))
    (`AudioComponent.SetVolumeMultiplier` _audio 1.0)
    (`AudioComponent.Play` _audio 0.0)))

(fn `UserConstructionScript`)
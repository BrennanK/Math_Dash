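; Level 5 corridor cross-section for a procedurally generated runner, randomly shaped forward, left or right by toggling connectors, walls and collision.
; BeginPlay also spawns lab hazards, props, forward coin rows and speed boosts at placeholder components, plus a random math problem.
; The player crossing ForwardSpawnBox spawns another copy at the chosen exit, or the end goal when BP_ProceduralBuilder flags it.
; The builder tracks segments, removing one when BP_Teacher hits the entry trigger.
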(event `Lightning spawn effect`
  (for _array_element (`|MakeArray` (`self.Lightning sphere`) (`self.Lightning sphere2`) (`self.Lightning sphere3`))
    (bind _returnvalue (`SceneComponent.K2_GetComponentToWorld` _array_element))
    (`|SpawnActorFromClass` "/Game/Blueprints/BP_SpeedBoost.BP_SpeedBoost_C" (`KismetMathLibrary.MakeTransform` (`KismetMathLibrary.MakeVector` (.x (.location _returnvalue)) (.y (.location _returnvalue)) (+ (.z (.location _returnvalue)) 250.0)) (.rotation _returnvalue)) "Undefined" "MultiplyWithRoot" null null)))

(event `Right floor coins spawn`)

(event `Forward Coins spawn`
  (bind _returnvalue (`KismetMathLibrary.RandomBool`))
  (if _returnvalue
    (for _array_element (`|MakeArray` (`self.Forward coins2`))
      (bind _returnvalue_2 (`SceneComponent.K2_GetComponentToWorld` _array_element))
      (bind _returnvalue_3 (`|SpawnActorFromClass` "/Game/Blueprints/CoinBP.CoinBP_C" (`KismetMathLibrary.MakeTransform` (`KismetMathLibrary.MakeVector` (.x (.location _returnvalue_2)) (.y (.location _returnvalue_2)) (.z (.location _returnvalue_2))) (.rotation _returnvalue_2)) "AdjustIfPossibleButAlwaysSpawn" "MultiplyWithRoot" null null))
      (`self.Coin instance` _returnvalue_3 (`KismetMathLibrary.RandomIntegerInRange` 1 7) 100.0))
    (elif _returnvalue
      (for _array_element_2 (`|MakeArray` (`self.Forward coins`))
        (bind _returnvalue_4 (`SceneComponent.K2_GetComponentToWorld` _array_element_2))
        (bind _returnvalue_5 (`|SpawnActorFromClass` "/Game/Blueprints/CoinBP.CoinBP_C" (`KismetMathLibrary.MakeTransform` (`KismetMathLibrary.MakeVector` (.x (.location _returnvalue_4)) (.y (.location _returnvalue_4)) (.z (.location _returnvalue_4))) (.rotation _returnvalue_4)) "AdjustIfPossibleButAlwaysSpawn" "MultiplyWithRoot" null null))
        (`self.Coin instance` _returnvalue_5 (`KismetMathLibrary.RandomIntegerInRange` 1 7) 100.0))
      (else
        (for _array_element_3 (`|MakeArray` (`self.Forward coins3`))
          (bind _returnvalue_6 (`SceneComponent.K2_GetComponentToWorld` _array_element_3))
          (bind _returnvalue_7 (`|SpawnActorFromClass` "/Game/Blueprints/CoinBP.CoinBP_C" (`KismetMathLibrary.MakeTransform` (`KismetMathLibrary.MakeVector` (.x (.location _returnvalue_6)) (.y (.location _returnvalue_6)) (.z (.location _returnvalue_6))) (.rotation _returnvalue_6)) "AdjustIfPossibleButAlwaysSpawn" "MultiplyWithRoot" null null))
          (`self.Coin instance` _returnvalue_7 (`KismetMathLibrary.RandomIntegerInRange` 1 7) 100.0))))))

(event `Wet floor spawn`
  (for (_array_element _array_index) (`|MakeArray` (`self.Wet floor`) (`self.Wet floor1`) (`self.Wet floor2`) (`self.Wet floor3`) (`self.Wet floor4`) (`self.Wet floor5`) (`self.Wet floor6`))
    (switch `int` _array_index
      (:`0`
        (bind _returnvalue (`SceneComponent.K2_GetComponentLocation` _array_element))
        (bind _returnvalue_2 (`SceneComponent.K2_GetComponentRotation` _array_element))
        (`|SpawnActorFromClass` "/Game/Blueprints/BP_Lab_stools1.BP_Lab_stools1_C" (`KismetMathLibrary.MakeTransform` _returnvalue _returnvalue_2 (1.5 1.5 1.5)) "Undefined" "MultiplyWithRoot" null null :!label _label))
      (:`1`
        (`|SpawnActorFromClass` "/Game/Blueprints/BP_Lab_stools2.BP_Lab_stools2_C" (`KismetMathLibrary.MakeTransform` _returnvalue _returnvalue_2 (1.5 1.5 1.5)) "Undefined" "MultiplyWithRoot" null null :!label _label_2))
      (:`2`
        (`|SpawnActorFromClass` "/Game/Blueprints/BP_Lab_stools3.BP_Lab_stools3_C" (`KismetMathLibrary.MakeTransform` _returnvalue _returnvalue_2 (1.5 1.5 1.5)) "Undefined" "MultiplyWithRoot" null null :!label _label_3))
      (:`3`
        (goto _label))
      (:`4`
        (goto _label_2))
      (:`5`
        (goto _label_3)))
    (`SceneComponent.SetVisibility` _array_element false false)
    (`PrimitiveComponent.SetCollisionEnabled` _array_element "NoCollision")))

(event `Backpack spawn`
  (for _array_element (`|MakeArray` (`self.Backpack1`) (`self.Backpack2`) (`self.Backpack3`) (`self.Backpack4`) (`self.Backpack5`) (`self.Backpack6`) (`self.Backpack7`) (`self.Backpack`) (`self.Backpack8`) (`self.Backpack9`) (`self.Backpack10`) (`self.Backpack11`) (`self.Backpack12`))
    (if (`SceneComponent.bVisible` _array_element)
      (`|SpawnActorFromClass` "/Game/Blueprints/BP_Backpack.BP_Backpack_C" (`KismetMathLibrary.MakeTransform` (`SceneComponent.K2_GetComponentLocation` _array_element) (struct) (0.5 0.5 0.5)) "DontSpawnIfColliding" "MultiplyWithRoot" null null)
      (`SceneComponent.SetVisibility` _array_element false false)
      (`PrimitiveComponent.SetCollisionEnabled` _array_element "NoCollision"))))

(event `Left floor coins spawn`)

(event `Random coin spawn`
  (switch `/Game/Blueprints/Turn_Directions` (`self.Turn directions ref`)
    (:`NewEnumerator0`
      (`self.Left floor coins spawn`))
    (:`NewEnumerator1`
      (`self.Right floor coins spawn`))
    (:`NewEnumerator2`
      (`self.Forward Coins spawn`))))

(event `Locker collision check`
  (bind _array (`|MakeArray` (`self.Lockers 5`) (`self.Lockers 4`) (`self.Lockers 9`) (`self.Lockers 13`) (`self.Lockers 16`) (`self.Lockers 31`) (`self.Lockers 44`) (`self.Lockers 45`) (`self.Lockers 51`) (`self.Lockers 53`) (`self.Lockers 54`) (`self.Lockers 34`) (`self.Lockers 57`) (`self.Lockers 62`)))
  (`|ExecutionSequence`
    (:`then_0`
      (for _array_element _array
        (`SceneComponent.SetVisibility` _array_element true false)))
    (:`then_1`
      (for _array_element_2 _array
        (if (`SceneComponent.bVisible` _array_element_2)
          (`PrimitiveComponent.SetCollisionEnabled` _array_element_2 "QueryAndPhysics")
          (else
            (`PrimitiveComponent.SetCollisionEnabled` _array_element_2 "NoCollision")))))))

(event `self.ReceiveBeginPlay`
  (`|ExecutionSequence`
    (:`then_0`
      (bind _outactors (`GameplayStatics.GetAllActorsOfClass` "/Game/ThirdPerson/Blueprints/BP_ThirdPersonCharacter.BP_ThirdPersonCharacter_C"))
      (set `self.PlayerRef` (`|GetArrayItem` _outactors))
      (bind _output_get (set `PrimitiveComponent.bGenerateOverlapEvents` (`KismetMathLibrary.RandomBool`) (`self.Turn box`)))
      (if (== _output_get false)
        (`self.Set up Forward Direction`)
        (else
          (`self.Setup Turn Direction`))))
    (:`then_1`
      (`self.Locker collision check`)
      (`self.Chemical spill spawn`)
      (`self.Science table spawn spawn`)
      (`self.Electrical cords spawn`)
      (`self.Wet floor spawn`)
      (`self.Forward Coins spawn`)
      (`self.Lightning spawn effect`))
    (:`then_2`
      (`self.Find Builder`))))

(event `Random left side wall`
  (switch `int` (`KismetMathLibrary.RandomIntegerInRange` 0 4)))

(event `self.Turn box.OnComponentBeginOverlap`
  (params (OverlappedComponent :type "PrimitiveComponent Object Reference") (OtherActor :type "Actor Object Reference") (OtherComp :type "PrimitiveComponent Object Reference") (OtherBodyIndex :type Integer) (bFromSweep :type Boolean) (SweepResult :type "HitResult Structure (by ref)"))
  (cast `/Game/ThirdPerson/Blueprints/BP_ThirdPersonCharacter` OtherActor))

(event `self.Left Segment Left side Math Problem Box collision.OnComponentBeginOverlap`
  (params (OverlappedComponent :type "PrimitiveComponent Object Reference") (OtherActor :type "Actor Object Reference") (OtherComp :type "PrimitiveComponent Object Reference") (OtherBodyIndex :type Integer) (bFromSweep :type Boolean) (SweepResult :type "HitResult Structure (by ref)"))
  ;[1 1 1] Spawns a Math Problem on the Left Side
)

(event `self.Forward spawn box.OnComponentBeginOverlap`
  (params (OverlappedComponent :type "PrimitiveComponent Object Reference") (OtherActor :type "Actor Object Reference") (OtherComp :type "PrimitiveComponent Object Reference") (OtherBodyIndex :type Integer) (bFromSweep :type Boolean) (SweepResult :type "HitResult Structure (by ref)"))
  ;[1 1 1] Procedural Generated Event for Cross Section
  (cast `/Game/ThirdPerson/Blueprints/BP_ThirdPersonCharacter` OtherActor)
  (switch `/Game/Blueprints/Turn_Directions` (`self.Turn directions ref`)
    (:`NewEnumerator0`
      (`self.Spawn Cross section at the Left End`))
    (:`NewEnumerator1`
      (`self.Spawn Cross Section at Right End`))
    (:`NewEnumerator2`
      (`self.Spawn Cross Section at the Forward end`))))

(event `self.Forward  Math Problem Box collision.OnComponentBeginOverlap`
  (params (OverlappedComponent :type "PrimitiveComponent Object Reference") (OtherActor :type "Actor Object Reference") (OtherComp :type "PrimitiveComponent Object Reference") (OtherBodyIndex :type Integer) (bFromSweep :type Boolean) (SweepResult :type "HitResult Structure (by ref)"))
  ;[1 1 1] Spawn A
)

(event `self.Right Segment Right side Math Problem Box collision.OnComponentBeginOverlap`
  (params (OverlappedComponent :type "PrimitiveComponent Object Reference") (OtherActor :type "Actor Object Reference") (OtherComp :type "PrimitiveComponent Object Reference") (OtherBodyIndex :type Integer) (bFromSweep :type Boolean) (SweepResult :type "HitResult Structure (by ref)")))

(event `self.Entry Destroy actor collision.OnComponentBeginOverlap`
  (params (OverlappedComponent :type "PrimitiveComponent Object Reference") (OtherActor :type "Actor Object Reference") (OtherComp :type "PrimitiveComponent Object Reference") (OtherBodyIndex :type Integer) (bFromSweep :type Boolean) (SweepResult :type "HitResult Structure (by ref)"))
  ;[1 1 1] This destoys the actor
  (cast `/Game/Blueprints/BP_Teacher` OtherActor)
  (`/Game/Blueprints/BP_ProceduralBuilder.Remove segment` (`self.Builder REF`)))

(event `Find Builder`
  (bind _outactors (`GameplayStatics.GetAllActorsOfClass` "/Game/Blueprints/BP_ProceduralBuilder.BP_ProceduralBuilder_C"))
  (set `self.Builder REF` (`|GetArrayItem` _outactors)))

(event `Science table spawn spawn`
  (for (_array_element _array_index) (`|MakeArray` (`self.BP_Science_Tables`) (`self.BP_Science_Tables1`) (`self.BP_Science_Tables2`) (`self.BP_Science_Tables3`) (`self.BP_Science_Tables4`) (`self.BP_Science_Tables5`) (`self.BP_Science_Tables6`) (`self.BP_Science_Tables7`) :!type "SceneComponent Object Reference")
    (if (`SceneComponent.bVisible` _array_element)
      (switch `int` _array_index
        (:`0`
          (bind _returnvalue (`SceneComponent.K2_GetComponentLocation` _array_element))
          (bind (_returnvalue_roll _returnvalue_pitch _returnvalue_yaw) (`KismetMathLibrary.BreakRotator` (`SceneComponent.K2_GetComponentRotation` _array_element)))
          (bind _returnvalue_2 (+ _returnvalue_yaw 0.0))
          (bind _relativescale3d (`SceneComponent.RelativeScale3D` _array_element))
          (bind _returnvalue_3 (`|SpawnActorFromClass` "/Game/Blueprints/BP_Science_Tables1.BP_Science_Tables1_C" (`KismetMathLibrary.MakeTransform` _returnvalue (`KismetMathLibrary.MakeRotator` _returnvalue_roll _returnvalue_pitch _returnvalue_2) _relativescale3d) "AdjustIfPossibleButAlwaysSpawn" "MultiplyWithRoot" null null))
          (`PrimitiveComponent.SetCollisionEnabled` (`/Game/Blueprints/BP_Science_Tables1.OpenFallenLocker1` _returnvalue_3) "NoCollision"))
        (:`1`
          (bind _returnvalue_4 (`|SpawnActorFromClass` "/Game/Blueprints/BP_Science_Tables3.BP_Science_Tables3_C" (`KismetMathLibrary.MakeTransform` _returnvalue (`KismetMathLibrary.MakeRotator` _returnvalue_roll _returnvalue_pitch _returnvalue_2) _relativescale3d) "AdjustIfPossibleButAlwaysSpawn" "MultiplyWithRoot" null null))
          (`PrimitiveComponent.SetCollisionEnabled` (`/Game/Blueprints/BP_Science_Tables3.OpenFallenLocker1` _returnvalue_4) "NoCollision"))
        (:`2`
          (bind _returnvalue_5 (`|SpawnActorFromClass` "/Game/Blueprints/BP_Science_Tables2.BP_Science_Tables2_C" (`KismetMathLibrary.MakeTransform` _returnvalue (`KismetMathLibrary.MakeRotator` _returnvalue_roll _returnvalue_pitch _returnvalue_2) _relativescale3d) "AdjustIfPossibleButAlwaysSpawn" "MultiplyWithRoot" null null))
          (`PrimitiveComponent.SetCollisionEnabled` (`/Game/Blueprints/BP_Science_Tables2.OpenFallenLocker1` _returnvalue_5) "NoCollision")))
      (`SceneComponent.SetVisibility` _array_element false false)
      (else
        (`SceneComponent.SetVisibility` _array_element true false)))))

(event `Chemical spill spawn`
  (`/Engine/EditorBlueprintResources/StandardMacros.DoOnce` false
    (:`Completed`
      (for (_array_element _array_index) (`|MakeArray` (`self.Entry Glue spill scene`) (`self.Entry Glue spill scene 2`) (`self.Entry floor spill scene 1`) (`self.Right floor Glue spill scene 3`) (`self.Right Glue spill scene 4`) (`self.Right floor Glue spill scene5`) (`self.forward Glue spill scene6`) (`self.forward Glue spill scene7`) (`self.Left Glue spill scene9`) (`self.left Glue spill scene10`) (`self.left Glue spill scene11`) (`self.forward Glue spill scene8`))
        (switch `int` _array_index
          (:`0`
            (bind _returnvalue (`SceneComponent.K2_GetComponentLocation` _array_element))
            (`|SpawnActorFromClass` "/Game/Blueprints/BP_Chemical_spills3.BP_Chemical_spills3_C" (`KismetMathLibrary.MakeTransform` _returnvalue (struct) (2.0 2.0 2.0)) "Undefined" "MultiplyWithRoot" null null :!label _label_4))
          (:`1`
            (`|SpawnActorFromClass` "/Game/Blueprints/BP_Chemical_spills1.BP_Chemical_spills1_C" (`KismetMathLibrary.MakeTransform` _returnvalue (struct) (2.0 2.0 2.0)) "Undefined" "MultiplyWithRoot" null null :!label _label_5))
          (:`2`
            (`|SpawnActorFromClass` "/Game/Blueprints/BP_Chemical_spills2.BP_Chemical_spills2_C" (`KismetMathLibrary.MakeTransform` _returnvalue (struct) (2.0 2.0 2.0)) "Undefined" "MultiplyWithRoot" null null :!label _label_6))
          (:`3`
            (goto _label_4))
          (:`4`
            (goto _label_5))
          (:`5`
            (goto _label_6)))))))

(event `Electrical cords spawn`
  (for (_array_element _array_index) (`|MakeArray` (`self.Shattered pages screen1`) (`self.Shattered pages screen`) (`self.Shattered pages screen2`) (`self.Shattered pages screen3`) (`self.Shattered pages screen4`) (`self.Shattered pages screen5`) (`self.Shattered pages screen6`) (`self.Shattered pages screen7`))
    (switch `int` _array_index
      (:`0`
        (bind _returnvalue (`SceneComponent.K2_GetComponentLocation` _array_element))
        (`|SpawnActorFromClass` "/Game/Blueprints/BP_Electrical_cords1.BP_Electrical_cords1_C" (`KismetMathLibrary.MakeTransform` _returnvalue (struct) (2.0 2.0 2.0)) "Undefined" "MultiplyWithRoot" null null :!label _label_7))
      (:`1`
        (`|SpawnActorFromClass` "/Game/Blueprints/BP_Electrical_cords2.BP_Electrical_cords2_C" (`KismetMathLibrary.MakeTransform` _returnvalue (struct) (2.0 2.0 2.0)) "Undefined" "MultiplyWithRoot" null null :!label _label_8))
      (:`2`
        (`|SpawnActorFromClass` "/Game/Blueprints/BP_Electrical_cords3.BP_Electrical_cords3_C" (`KismetMathLibrary.MakeTransform` _returnvalue (struct) (2.0 2.0 2.0)) "Undefined" "MultiplyWithRoot" null null :!label _label_9))
      (:`3`
        (goto _label_7))
      (:`4`
        (goto _label_8))
      (:`5`
        (goto _label_9)))))

(fn `Calculate Forward location and Rotation`
  (returns (ReturnValue :type "Vector Structure") (ReturnValue2 :type "Rotator Structure"))
  (return (+ (`SceneComponent.K2_GetComponentLocation` (`self.Forward floor`)) (* (`self.GetActorForwardVector`) (`self.Gap value`))) (`self.K2_GetActorRotation`)))

(fn `Calculate Left Location and Rotation`
  (returns (ReturnValue :type "Vector Structure") (ReturnValue_Roll :type "Float (single-precision)") (ReturnValue_Pitch :type "Float (single-precision)") (ReturnValue2 :type "Float (double-precision)"))
  (bind (_returnvalue_roll _returnvalue_pitch _returnvalue_yaw) (`KismetMathLibrary.BreakRotator` (`self.K2_GetActorRotation`)))
  (return (+ (`SceneComponent.K2_GetComponentLocation` (`self.Left Segment Leftfloor`)) (* (* (`self.GetActorRightVector`) -1.0) (`self.Gap value`))) _returnvalue_roll _returnvalue_pitch (- _returnvalue_yaw 90.0)))

(fn `Calculate Right Location and Rotation`
  (returns (ReturnValue :type "Vector Structure") (ReturnValue_Roll :type "Float (single-precision)") (ReturnValue_Pitch :type "Float (single-precision)") (ReturnValue2 :type "Float (double-precision)"))
  (bind (_returnvalue_roll _returnvalue_pitch _returnvalue_yaw) (`KismetMathLibrary.BreakRotator` (`self.K2_GetActorRotation`)))
  (return (+ (`SceneComponent.K2_GetComponentLocation` (`self.Right Segment Right Floor`)) (* (`self.GetActorRightVector`) (`self.Gap value`))) _returnvalue_roll _returnvalue_pitch (+ _returnvalue_yaw 90.0)))

(fn `Coin instance`
  (params (`Coin REF` :type "/Game/Blueprints/CoinBP Object Reference") (`number of coins ` :type Integer :default 0) (`space between coins` :type "Float (double-precision)" :default 200.0))
  (bind (_returnvalue_location _returnvalue_rotation _returnvalue_scale) (`KismetMathLibrary.BreakTransform` (`self.GetTransform` `Coin REF`)))
  (for _index (range 1 (+ `number of coins ` 1))
    (`|SpawnActorFromClass` (`GameplayStatics.GetObjectClass` `Coin REF`) (`KismetMathLibrary.MakeTransform` (+ _returnvalue_location (* (`self.GetActorForwardVector` `Coin REF`) `space between coins` _index)) _returnvalue_rotation _returnvalue_scale) "Undefined" "MultiplyWithRoot" null null)))

(fn `Decide to Spawn A math Problem`
  (params (Direction :type "/Game/Blueprints/Turn_Directions Enum" :default "NewEnumerator0"))
  (locals (`Spawn Forward Problem` :type Boolean) (`Spawn Left Problem` :type Boolean) (`Spawn Right Problem` :type Boolean))
  (switch `/Game/Blueprints/Turn_Directions` Direction
    (:`NewEnumerator0`
      (bind _output_get (set `local.Spawn Left Problem` (`KismetMathLibrary.RandomBool`)))
      (if _output_get
        (`|SpawnActorFromClass` "/Game/Blueprints/MathProblem_UI.MathProblem_UI_C" (`SceneComponent.K2_GetComponentToWorld` (`self.Left Segment Left side Math Problem Box collision`)) "Undefined" "MultiplyWithRoot" null null)))
    (:`NewEnumerator1`
      (bind _output_get_2 (set `local.Spawn Right Problem` (`KismetMathLibrary.RandomBool`)))
      (if _output_get_2
        (`|SpawnActorFromClass` "/Game/Blueprints/MathProblem_UI.MathProblem_UI_C" (`SceneComponent.K2_GetComponentToWorld` (`self.Right Segment Right side Math Problem Box collision`)) "Undefined" "MultiplyWithRoot" null null)))
    (:`NewEnumerator2`
      (bind _output_get_3 (set `local.Spawn Forward Problem` (`KismetMathLibrary.RandomBool`)))
      (if _output_get_3
        (`|SpawnActorFromClass` "/Game/Blueprints/MathProblem_UI.MathProblem_UI_C" (`SceneComponent.K2_GetComponentToWorld` (`self.Forward  Math Problem Box collision`)) "Undefined" "MultiplyWithRoot" null null)))))

(fn `Set up Forward Direction`
  (bind _left_segment_leftfloor (`self.Left Segment Leftfloor`))
  (bind _left_segment_right_wall_right_side (`self.Left Segment Right Wall Right side`))
  (bind _left_segment_leftwall_left_side (`self.Left Segment Leftwall left side`))
  (bind _right_segment_right_floor (`self.Right Segment Right Floor`))
  (bind _right_segment_rightfllor_right_side (`self.Right Segment Rightfllor Right Side`))
  (bind _right_segment__left_wall_left_side (`self.Right Segment  Left wall left side`))
  (`SceneComponent.SetVisibility` (`self.Cube`) false false)
  (`SceneComponent.SetVisibility` (`self.Forward connector`) true true)
  (`PrimitiveComponent.SetCollisionEnabled` (`self.Forward_Left_wall_connector`) "QueryAndPhysics")
  (`PrimitiveComponent.SetCollisionEnabled` (`self.Forward_right_wall_connector`) "QueryAndPhysics")
  (`|ExecutionSequence`
    (:`then_0`
      (`|ExecutionSequence`
        (:`then_0`
          (`SceneComponent.SetVisibility` _left_segment_leftfloor false false)
          (`SceneComponent.SetVisibility` _left_segment_right_wall_right_side false false)
          (`SceneComponent.SetVisibility` _left_segment_leftwall_left_side false false))
        (:`then_1`
          (`PrimitiveComponent.SetCollisionEnabled` _left_segment_leftfloor "NoCollision")
          (`PrimitiveComponent.SetCollisionEnabled` _left_segment_right_wall_right_side "NoCollision")
          (`PrimitiveComponent.SetCollisionEnabled` _left_segment_leftwall_left_side "QueryAndPhysics"))))
    (:`then_1`
      (`|ExecutionSequence`
        (:`then_0`
          (`SceneComponent.SetVisibility` _right_segment_right_floor false false)
          (`SceneComponent.SetVisibility` _right_segment_rightfllor_right_side false false)
          (`SceneComponent.SetVisibility` _right_segment__left_wall_left_side false false))
        (:`then_1`
          (`PrimitiveComponent.SetCollisionEnabled` _right_segment_right_floor "QueryAndPhysics")
          (`PrimitiveComponent.SetCollisionEnabled` _right_segment_rightfllor_right_side "QueryAndPhysics")
          (`PrimitiveComponent.SetCollisionEnabled` _right_segment__left_wall_left_side "QueryAndPhysics"))))
    (:`then_2`
      (set `self.Turn directions ref` "NewEnumerator2"))
    (:`then_3`
      (`self.Decide to Spawn A math Problem` "NewEnumerator2"))))

(fn `Setup Turn Direction`
  (bind _left_segment_leftfloor (`self.Left Segment Leftfloor`))
  (bind _left_segment_right_wall_right_side (`self.Left Segment Right Wall Right side`))
  (bind _left_segment_leftwall_left_side (`self.Left Segment Leftwall left side`))
  (bind _right_segment_right_floor (`self.Right Segment Right Floor`))
  (bind _right_segment_rightfllor_right_side (`self.Right Segment Rightfllor Right Side`))
  (bind _right_segment__left_wall_left_side (`self.Right Segment  Left wall left side`))
  (bind _left_connector (`self.Left connector`))
  (bind _right_connector (`self.right connector`))
  (bind _returnvalue (`|SpawnActorFromClass` "/Game/Blueprints/Turn_Collision.Turn_Collision_C" (`SceneComponent.K2_GetComponentToWorld` (`self.Turn box`)) "Undefined" "MultiplyWithRoot" null null))
  (`BoxComponent.SetBoxExtent` (`/Game/Blueprints/Turn_Collision.Box` _returnvalue) (`BoxComponent.BoxExtent` (`self.Turn box`)) true)
  (switch `int` (`KismetMathLibrary.RandomIntegerInRange` (`self.Random integer`) 1)
    (:`0`
      (set `/Game/Blueprints/Turn_Collision.Left Or Right` "NewEnumerator1" _returnvalue)
      (`|ExecutionSequence`
        (:`then_0`
          (`SceneComponent.SetVisibility` _left_segment_leftfloor false false)
          (`SceneComponent.SetVisibility` _left_segment_right_wall_right_side false false)
          (`SceneComponent.SetVisibility` _left_segment_leftwall_left_side false false)
          (`SceneComponent.SetVisibility` _right_connector true true))
        (:`then_1`
          (`PrimitiveComponent.SetCollisionEnabled` _left_segment_leftfloor "NoCollision")
          (`PrimitiveComponent.SetCollisionEnabled` _left_segment_right_wall_right_side "NoCollision")
          (`PrimitiveComponent.SetCollisionEnabled` _left_segment_leftwall_left_side "NoCollision")
          (`PrimitiveComponent.SetCollisionEnabled` _right_connector "NoCollision")
          (`PrimitiveComponent.SetCollisionEnabled` (`self.Right_connector_left_wall_connector`) "QueryAndPhysics")
          (`PrimitiveComponent.SetCollisionEnabled` (`self.Right_connector_front_wall_connector`) "QueryAndPhysics"))
        (:`then_2`
          (set `self.Turn directions ref` "NewEnumerator1"))
        (:`then_3`
          (`self.Decide to Spawn A math Problem` "NewEnumerator1"))))
    (:`1`
      (set `/Game/Blueprints/Turn_Collision.Left Or Right` "NewEnumerator0" _returnvalue)
      (`|ExecutionSequence`
        (:`then_0`
          (`SceneComponent.SetVisibility` _right_segment_right_floor false false)
          (`SceneComponent.SetVisibility` _right_segment_rightfllor_right_side false false)
          (`SceneComponent.SetVisibility` _right_segment__left_wall_left_side false false)
          (`SceneComponent.SetVisibility` _left_connector true true))
        (:`then_1`
          (`PrimitiveComponent.SetCollisionEnabled` _right_segment_right_floor "NoCollision")
          (`PrimitiveComponent.SetCollisionEnabled` _right_segment_rightfllor_right_side "NoCollision")
          (`PrimitiveComponent.SetCollisionEnabled` _right_segment__left_wall_left_side "NoCollision")
          (`PrimitiveComponent.SetCollisionEnabled` _left_connector "NoCollision")
          (`PrimitiveComponent.SetCollisionEnabled` (`self.Left_Cnnector_wall_connector`) "QueryAndPhysics")
          (`PrimitiveComponent.SetCollisionEnabled` (`self.Left_Cnnector_wall_connector2`) "QueryAndPhysics"))
        (:`then_2`
          (set `self.Turn directions ref` "NewEnumerator0"))
        (:`then_3`
          (`self.Decide to Spawn A math Problem` "NewEnumerator0"))))))

(fn `Spawn Cross Section at Right End`
  (if (`/Game/Blueprints/BP_ProceduralBuilder.SpawnEndGoal?` (`self.Builder REF`))
    (set `self.Gap value` 2100.0)
    (bind (_returnvalue _returnvalue_roll _returnvalue_pitch _returnvalue2) (`self.Calculate Right Location and Rotation`))
    (`|SpawnActorFromClass` "/Game/Blueprints/BP_Spawn_Endgoal.BP_Spawn_Endgoal_C" (`KismetMathLibrary.MakeTransform` _returnvalue (`KismetMathLibrary.MakeRotator` _returnvalue_roll _returnvalue_pitch _returnvalue2)) "Undefined" "MultiplyWithRoot" null null)
    (else
      (bind (_returnvalue_2 _returnvalue_roll_2 _returnvalue_pitch_2 _returnvalue2_2) (`self.Calculate Right Location and Rotation`))
      (bind _returnvalue_3 (`|SpawnActorFromClass` (`GameplayStatics.GetObjectClass` self) (`KismetMathLibrary.MakeTransform` (- _returnvalue_2 (`self.Offset`)) (`KismetMathLibrary.MakeRotator` _returnvalue_roll_2 _returnvalue_pitch_2 _returnvalue2_2)) "Undefined" "MultiplyWithRoot" null null))
      (`/Game/Blueprints/BP_ProceduralBuilder.Add to Segments` (`self.Builder REF`) _returnvalue_3))))

(fn `Spawn Cross Section at the Forward end`
  (if (`/Game/Blueprints/BP_ProceduralBuilder.SpawnEndGoal?` (`self.Builder REF`))
    (set `self.Gap value` 2100.0)
    (bind (_returnvalue _returnvalue2) (`self.Calculate Forward location and Rotation`))
    (`|SpawnActorFromClass` "/Game/Blueprints/BP_Spawn_Endgoal.BP_Spawn_Endgoal_C" (`KismetMathLibrary.MakeTransform` _returnvalue _returnvalue2) "Undefined" "MultiplyWithRoot" null null)
    (else
      (bind (_returnvalue_2 _returnvalue2_2) (`self.Calculate Forward location and Rotation`))
      (bind _returnvalue_3 (`|SpawnActorFromClass` (`GameplayStatics.GetObjectClass` self) (`KismetMathLibrary.MakeTransform` (- _returnvalue_2 (`self.Offset`)) _returnvalue2_2) "Undefined" "MultiplyWithRoot" null null))
      (`/Game/Blueprints/BP_ProceduralBuilder.Add to Segments` (`self.Builder REF`) _returnvalue_3))))

(fn `Spawn Cross section at the Left End`
  (if (`/Game/Blueprints/BP_ProceduralBuilder.SpawnEndGoal?` (`self.Builder REF`))
    (set `self.Gap value` 2100.0)
    (bind (_returnvalue _returnvalue_roll _returnvalue_pitch _returnvalue2) (`self.Calculate Left Location and Rotation`))
    (`|SpawnActorFromClass` "/Game/Blueprints/BP_Spawn_Endgoal.BP_Spawn_Endgoal_C" (`KismetMathLibrary.MakeTransform` _returnvalue (`KismetMathLibrary.MakeRotator` _returnvalue_roll _returnvalue_pitch _returnvalue2)) "Undefined" "MultiplyWithRoot" null null)
    (else
      (bind (_returnvalue_2 _returnvalue_roll_2 _returnvalue_pitch_2 _returnvalue2_2) (`self.Calculate Left Location and Rotation`))
      (bind _returnvalue_3 (`|SpawnActorFromClass` (`GameplayStatics.GetObjectClass` self) (`KismetMathLibrary.MakeTransform` (- _returnvalue_2 (`self.Offset`)) (`KismetMathLibrary.MakeRotator` _returnvalue_roll_2 _returnvalue_pitch_2 _returnvalue2_2)) "Undefined" "MultiplyWithRoot" null null))
      (`/Game/Blueprints/BP_ProceduralBuilder.Add to Segments` (`self.Builder REF`) _returnvalue_3))))

(fn `UserConstructionScript`)
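; Wallet Blueprint that holds a Coins balance and provides functions to add, check and spend it.
; AddFunds increases Coins, and CheckAffordability sets Affordable by comparing a cost against the balance.
; SubtractFunds deducts the cost only when CheckAffordability returns true.
; As written, CheckAffordability always returns false regardless of Affordable, so SubtractFunds never deducts coins.
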(fn `Add Funds`
  (params (CoinsIn :type Integer))
  (set `self.Coins` (+ CoinsIn (`self.Coins`))))

(fn `Check Affordability`
  (params (cost :type Integer))
  (returns (result :type Boolean))
  (locals (Affordable :type Boolean))
  (if (<= cost (`self.Coins`))
    (set `local.Affordable` true)
    (else
      (set `local.Affordable` false)))
  (return false))

(fn `Subtract Funds`
  (params (Cost :type Integer))
  (bind _result (`self.Check Affordability` Cost))
  (if _result
    (set `self.Coins` (- (`self.Coins`) (`local.Cost`)))))
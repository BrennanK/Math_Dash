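; Procedural builder that tracks the level's cross-section segments in an ordered list, seeded with a starting section on BeginPlay.
; AddToSegments appends segments and counts them, setting SpawnEndGoal when the count reaches LimitBeforeEndGoalSpawns.
; RemoveSegment drops the oldest segment, messaging it to destroy its spawned actors before destroying it, with a debug print.
; Segment spawning happens outside this Blueprint.
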(event `self.ReceiveBeginPlay`
  (`KismetArrayLibrary.Array_Add` (`self.Cross section segments`) (`self.Starting Section`)))

(fn `Add to Segments`
  (params (`Segment add` :type "Actor Object Reference"))
  (bind _number_of_segments_added (`self.Number of Segments added`))
  (`KismetArrayLibrary.Array_Add` (`self.Cross section segments`) `Segment add`)
  (`/Engine/EditorBlueprintResources/StandardMacros.IncrementInt` _number_of_segments_added
    (:`  `
      (if (== (`self.Limit before End Goal spawns`) _number_of_segments_added)
        (set `self.SpawnEndGoal?` true)))))

(fn `Cast and Destroy`
  (params (`Segment to Cast` :type "Actor Object Reference"))
  (message `/Game/Blueprints/BPI_Cross_Section.Signal Destructionof Spawned Actors` `Segment to Cast`))

(fn `Remove segment`
  (bind _output (`|GetArrayItem` (`self.Cross section segments`)))
  (`KismetSystemLibrary.PrintString` (`KismetSystemLibrary.GetDisplayName` _output) true true (struct :`R` 1.0 :`G` 0.016606 :`A` 1.0) 12.0)
  (`self.Cast and Destroy` _output)
  (`self.K2_DestroyActor` _output)
  (`KismetArrayLibrary.Array_Remove` (`self.Cross section segments`)))

(fn `UserConstructionScript`)
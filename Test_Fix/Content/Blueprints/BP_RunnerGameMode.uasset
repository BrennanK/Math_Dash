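; BP_RunnerGameMode is a runner game mode that builds and recycles an endless floor from BP_Floor tiles.
; On BeginPlay it spawns NumberOfTiles tiles, each placed at the previous tile's attach point and tracked in FloorTiles.
; ExtendFloor appends another tile and destroys the oldest once the count exceeds NumberOfTiles plus a small buffer, keeping the track length bounded.
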(event `self.ReceiveBeginPlay`
  (for _ (range (`self.numberOfTiles`))
    (`self.AddFloor`)))

(fn `AddFloor`
  (bind _returnvalue (`|SpawnActorFromClass` "/Game/Blueprints/BP_Floor.BP_Floor_C" (`self.floorAttachPoint`) "Undefined" "MultiplyWithRoot" null null))
  (bind _returnvalue_2 (`/Game/Blueprints/BP_Floor.GetAttachPoint` _returnvalue))
  (set `self.floorAttachPoint` _returnvalue_2)
  (`KismetArrayLibrary.Array_Add` (`self.floorTiles`) _returnvalue))

(fn `ExtendFloor`
  (bind _floortiles (`self.floorTiles`))
  (bind _output (`|GetArrayItem` _floortiles))
  (`self.AddFloor`)
  (if (> (`KismetArrayLibrary.Array_Length` (`self.floorTiles`)) (+ (`self.numberOfTiles`) 2))
    (`self.K2_DestroyActor` _output)
    (`KismetArrayLibrary.Array_RemoveItem` _floortiles _output)))

(fn `UserConstructionScript`)
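; CoinBP is a collectible coin actor that spins and is picked up when the third-person character overlaps its sphere.
; A looping 60 Hz timer, rather than Tick, increments the coin's yaw.
; On pickup it plays the coin sound, passes its own CoinScore, unchanged by an add of zero, to the player UI's UpdateCoinCount, then clears the timer and destroys itself.
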(event `self.ReceiveBeginPlay`
  (bind _returnvalue (`KismetSystemLibrary.K2_SetTimer` null "Rotate Coin" (/ 1.0 60.0) true))
  (set `self.Rotate Timer` _returnvalue))

(event `self.ReceiveTick`
  (params (DeltaSeconds :type "Float (single-precision)")))

(event `Rotate Coin`
  (bind (_returnvalue_roll _returnvalue_pitch _returnvalue_yaw) (`KismetMathLibrary.BreakRotator` (`self.K2_GetActorRotation`)))
  (`self.K2_SetActorRotation` (`KismetMathLibrary.MakeRotator` _returnvalue_roll _returnvalue_pitch (+ _returnvalue_yaw 1.0))))

(event `self.sphere.OnComponentBeginOverlap`
  (params (OverlappedComponent :type "PrimitiveComponent Object Reference") (OtherActor :type "Actor Object Reference") (OtherComp :type "PrimitiveComponent Object Reference") (OtherBodyIndex :type Integer) (bFromSweep :type Boolean) (SweepResult :type "HitResult Structure (by ref)"))
  (bind _sfx_coin (`self.SFX_Coin`))
  (bind _asbp_third_person_character (cast `/Game/ThirdPerson/Blueprints/BP_ThirdPersonCharacter` OtherActor))
  (`AudioComponent.SetVolumeMultiplier` _sfx_coin 1.0)
  (`AudioComponent.Play` _sfx_coin 0.0)
  (bind _output_get (set `self.Coin score` (+ (`self.Coin score`) 0)))
  (`/Game/Characters/Player_UI/W_MainPlayer.Update coin count` (`/Game/ThirdPerson/Blueprints/BP_ThirdPersonCharacter.Player UI Ref` _asbp_third_person_character) _output_get)
  (`KismetSystemLibrary.K2_ClearAndInvalidateTimerHandle` (`self.Rotate Timer`))
  (`self.K2_DestroyActor`))

(fn `UserConstructionScript`)
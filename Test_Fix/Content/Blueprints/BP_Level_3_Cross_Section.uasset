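; Procedural cross-section segment for Level 3 that chains copies of itself as the player advances.
; On BeginPlay it picks a random in-bounds direction, configures walls and turn collision, maybe spawns a math problem, and swaps placeholder components for obstacles, coins and lightning effects.
; Player overlap with ForwardSpawnBox spawns the next segment or, when BP_ProceduralBuilder signals, the end goal.
; BP_Teacher overlap at the entry has the builder remove a segment.
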(event `Lightning spawn effect`
  (bind _class (`self.Class`))
  (for _array_element (`|MakeArray` (`self.Lightning sphere`) (`self.Lightning sphere2`) (`self.Lightning sphere3`))
    (bind _returnvalue (`SceneComponent.K2_GetComponentToWorld` _array_element))
    (`|SpawnActorFromClass` (`|GetArrayItem` _class (`KismetMathLibrary.RandomIntegerInRange` 0 (- (`KismetArrayLibrary.Array_Length` _class) 1))) (`KismetMathLibrary.MakeTransform` (`KismetMathLibrary.MakeVector` (.x (.location _returnvalue)) (.y (.location _returnvalue)) (.z (.location _returnvalue))) (.rotation _returnvalue)) "Undefined" "MultiplyWithRoot" null null)))

(event `Right floor coins spawn`)

(event `Forward Coins spawn`
  (bind _array (`|MakeArray` (`self.Forward Coin`) (`self.Forward Coin2`) (`self.Forward Coin3`)))
  (bind _output_get (set `self.Right Random Coin` (`KismetMathLibrary.RandomIntegerInRange` 0 (- (`KismetArrayLibrary.Array_Length` _array) 1))))
  (for (_array_element _array_index) _array
    (if (== _output_get _array_index)
      (bind (_returnvalue_location _returnvalue_rotation) (`KismetMathLibrary.BreakTransform` (`SceneComponent.K2_GetComponentToWorld` _array_element)))
      (bind _returnvalue (`|SpawnActorFromClass` "/Game/Blueprints/CoinBP.CoinBP_C" (`KismetMathLibrary.MakeTransform` _returnvalue_location _returnvalue_rotation) "Undefined" "MultiplyWithRoot" null null))
      (`ActorComponent.K2_DestroyComponent` _array_element)
      (`self.Coin instance` _returnvalue (`KismetMathLibrary.RandomIntegerInRange` 1 7) 100.0)
      (else
        (`ActorComponent.K2_DestroyComponent` _array_element)))))

(event `Wet floor spawn`
  (for _array_element (`|MakeArray` (`self.Wet floor`) (`self.Wet floor1`) (`self.Wet floor2`) (`self.Wet floor3`) (`self.Wet floor4`) (`self.Wet floor5`) (`self.Wet floor6`))
    (`|SpawnActorFromClass` "/Game/Blueprints/BP_Trash_Can.BP_Trash_Can_C" (`KismetMathLibrary.MakeTransform` (`SceneComponent.K2_GetComponentLocation` _array_element) (`SceneComponent.K2_GetComponentRotation` _array_element)) "Undefined" "MultiplyWithRoot" null null)
    (`SceneComponent.SetVisibility` _array_element false false)
    (`PrimitiveComponent.SetCollisionEnabled` _array_element "NoCollision")))

(event `Backpack spawn`)

(event `Left floor coins spawn`)

(event `Random coin spawn`
  (switch `/Game/Blueprints/Turn_Directions` (`self.Turn directions ref`)
    (:`NewEnumerator0`
      (`self.Left floor coins spawn`))
    (:`NewEnumerator1`
      (`self.Right floor coins spawn`))
    (:`NewEnumerator2`
      (`self.Forward Coins spawn`))))

(event `Locker collision check`)

(event `self.ReceiveBeginPlay`
  (`|ExecutionSequence`
    (:`then_0`
      (bind _outactors (`GameplayStatics.GetAllActorsOfClass` "/Game/ThirdPerson/Blueprints/BP_ThirdPersonCharacter.BP_ThirdPersonCharacter_C"))
      (set `self.PlayerRef` (`|GetArrayItem` _outactors))
      (`self.Decide What Segment To Do Next`))
    (:`then_1`
      (`self.Locker collision check`)
      (`self.Glue spill spawn`)
      (`self.Fallen lockers spawn`)
      (`self.shattered papers spawn`)
      (`self.Wet floor spawn`)
      (`self.Forward Coins spawn`)
      (`self.Lightning spawn effect`))
    (:`then_2`
      (`self.Find Builder`))))

(event `Random left side wall`
  (switch `int` (`KismetMathLibrary.RandomIntegerInRange` 0 4)))

(event `self.Turn box.OnComponentBeginOverlap`
  (params (OverlappedComponent :type "PrimitiveComponent Object Reference") (OtherActor :type "Actor Object Reference") (OtherComp :type "PrimitiveComponent Object Reference") (OtherBodyIndex :type Integer) (bFromSweep :type Boolean) (SweepResult :type "HitResult Structure (by ref)"))
  (cast `/Game/ThirdPerson/Blueprints/BP_ThirdPersonCharacter` OtherActor))

(event `self.Left Segment Left side Math Problem Box collision.OnComponentBeginOverlap`
  (params (OverlappedComponent :type "PrimitiveComponent Object Reference") (OtherActor :type "Actor Object Reference") (OtherComp :type "PrimitiveComponent Object Reference") (OtherBodyIndex :type Integer) (bFromSweep :type Boolean) (SweepResult :type "HitResult Structure (by ref)"))
  ;[1 1 1] Spawns a Math Problem on the Left Side
)

(event `self.Forward spawn box.OnComponentBeginOverlap`
  (params (OverlappedComponent :type "PrimitiveComponent Object Reference") (OtherActor :type "Actor Object Reference") (OtherComp :type "PrimitiveComponent Object Reference") (OtherBodyIndex :type Integer) (bFromSweep :type Boolean) (SweepResult :type "HitResult Structure (by ref)"))
  ;[1 1 1] Procedural Generated Event for Cross Section
  (cast `/Game/ThirdPerson/Blueprints/BP_ThirdPersonCharacter` OtherActor)
  (switch `/Game/Blueprints/Turn_Directions` (`self.Turn directions ref`)
    (:`NewEnumerator0`
      (`self.Spawn Cross section at the Left End`))
    (:`NewEnumerator1`
      (`self.Spawn Cross Section at Right End`))
    (:`NewEnumerator2`
      (`self.Spawn Cross Section at the Forward end`))))

(event `self.Forward  Math Problem Box collision.OnComponentBeginOverlap`
  (params (OverlappedComponent :type "PrimitiveComponent Object Reference") (OtherActor :type "Actor Object Reference") (OtherComp :type "PrimitiveComponent Object Reference") (OtherBodyIndex :type Integer) (bFromSweep :type Boolean) (SweepResult :type "HitResult Structure (by ref)"))
  ;[1 1 1] Spawn A
)

(event `self.Right Segment Right side Math Problem Box collision.OnComponentBeginOverlap`
  (params (OverlappedComponent :type "PrimitiveComponent Object Reference") (OtherActor :type "Actor Object Reference") (OtherComp :type "PrimitiveComponent Object Reference") (OtherBodyIndex :type Integer) (bFromSweep :type Boolean) (SweepResult :type "HitResult Structure (by ref)")))

(event `self.Entry Destroy actor collision.OnComponentBeginOverlap`
  (params (OverlappedComponent :type "PrimitiveComponent Object Reference") (OtherActor :type "Actor Object Reference") (OtherComp :type "PrimitiveComponent Object Reference") (OtherBodyIndex :type Integer) (bFromSweep :type Boolean) (SweepResult :type "HitResult Structure (by ref)"))
  ;[1 1 1] This destoys the actor
  (cast `/Game/Blueprints/BP_Teacher` OtherActor)
  (`/Game/Blueprints/BP_ProceduralBuilder.Remove segment` (`self.Builder REF`)))

(event `Find Builder`
  (bind _outactors (`GameplayStatics.GetAllActorsOfClass` "/Game/Blueprints/BP_ProceduralBuilder.BP_ProceduralBuilder_C"))
  (set `self.Builder REF` (`|GetArrayItem` _outactors)))

(event `Glue spill spawn`
  (for _array_element (`|MakeArray` (`self.FoodSpill5`) (`self.FoodSpill6`) (`self.FoodSpill7`) (`self.FoodSpill8`) (`self.FoodSpill9`) (`self.FoodSpill10`) (`self.FoodSpill4`) (`self.FoodSpill`) (`self.FoodSpill1`) (`self.FoodSpill2`) (`self.FoodSpill3`) (`self.FoodSpill11`))
    (`|SpawnActorFromClass` "/Game/Blueprints/BP_Food_Spill.BP_Food_Spill_C" (`KismetMathLibrary.MakeTransform` (`SceneComponent.K2_GetComponentLocation` _array_element) (`SceneComponent.K2_GetComponentRotation` _array_element)) "Undefined" "MultiplyWithRoot" null null)
    (`ActorComponent.K2_DestroyComponent` _array_element)))

(event `Fallen lockers spawn`)

(event `shattered papers spawn`
  (for _array_element (`|MakeArray` (`self.SpilledTrays1`) (`self.SpilledTrays2`) (`self.SpilledTrays3`) (`self.SpilledTrays4`) (`self.SpilledTrays5`) (`self.SpilledTrays6`) (`self.SpilledTrays7`) (`self.SpilledTrays`))
    (`|SpawnActorFromClass` "/Game/Blueprints/BP_Spilled_Trays.BP_Spilled_Trays_C" (`KismetMathLibrary.MakeTransform` (`SceneComponent.K2_GetComponentLocation` _array_element) (`SceneComponent.K2_GetComponentRotation` _array_element)) "Undefined" "MultiplyWithRoot" null null)
    (`ActorComponent.K2_DestroyComponent` _array_element)))

(fn `Calculate Forward location and Rotation`
  (returns (ReturnValue :type "Vector Structure") (ReturnValue2 :type "Rotator Structure"))
  (return (+ (`SceneComponent.K2_GetComponentLocation` (`self.Forward floor`)) (* (`self.GetActorForwardVector`) (`self.Gap value`))) (`self.K2_GetActorRotation`)))

(fn `Calculate Left Location and Rotation`
  (returns (ReturnValue :type "Vector Structure") (ReturnValue_Roll :type "Float (single-precision)") (ReturnValue_Pitch :type "Float (single-precision)") (ReturnValue2 :type "Float (double-precision)"))
  (bind (_returnvalue_roll _returnvalue_pitch _returnvalue_yaw) (`KismetMathLibrary.BreakRotator` (`self.K2_GetActorRotation`)))
  (return (+ (`SceneComponent.K2_GetComponentLocation` (`self.Left Segment Leftfloor`)) (* (* (`self.GetActorRightVector`) -1.0) (`self.Gap value`))) _returnvalue_roll _returnvalue_pitch (- _returnvalue_yaw 90.0)))

(fn `Calculate Right Location and Rotation`
  (returns (ReturnValue :type "Vector Structure") (ReturnValue_Roll :type "Float (single-precision)") (ReturnValue_Pitch :type "Float (single-precision)") (ReturnValue2 :type "Float (double-precision)"))
  (bind (_returnvalue_roll _returnvalue_pitch _returnvalue_yaw) (`KismetMathLibrary.BreakRotator` (`self.K2_GetActorRotation`)))
  (return (+ (`SceneComponent.K2_GetComponentLocation` (`self.Right Segment Right Floor`)) (* (`self.GetActorRightVector`) (`self.Gap value`))) _returnvalue_roll _returnvalue_pitch (+ _returnvalue_yaw 90.0)))

(fn `Coin instance`
  (params (`Coin REF` :type "/Game/Blueprints/CoinBP Object Reference") (`number of coins ` :type Integer :default 0) (`space between coins` :type "Float (double-precision)" :default 200.0))
  (bind (_returnvalue_location _returnvalue_rotation _returnvalue_scale) (`KismetMathLibrary.BreakTransform` (`self.GetTransform` `Coin REF`)))
  (for _index (range 1 (+ `number of coins ` 1))
    (`|SpawnActorFromClass` (`GameplayStatics.GetObjectClass` `Coin REF`) (`KismetMathLibrary.MakeTransform` (+ _returnvalue_location (* (`self.GetActorForwardVector` `Coin REF`) `space between coins` _index)) _returnvalue_rotation _returnvalue_scale) "Undefined" "MultiplyWithRoot" null null)))

(fn `Decide to Spawn A math Problem`
  (params (Direction :type "/Game/Blueprints/Turn_Directions Enum" :default "NewEnumerator0"))
  (locals (`Spawn Forward Problem` :type Boolean) (`Spawn Left Problem` :type Boolean) (`Spawn Right Problem` :type Boolean))
  (switch `/Game/Blueprints/Turn_Directions` Direction
    (:`NewEnumerator0`
      (bind _output_get (set `local.Spawn Left Problem` (`KismetMathLibrary.RandomBool`)))
      (if _output_get
        (`|SpawnActorFromClass` "/Game/Blueprints/MathProblem_UI.MathProblem_UI_C" (`SceneComponent.K2_GetComponentToWorld` (`self.Left Segment Left side Math Problem Box collision`)) "Undefined" "MultiplyWithRoot" null null)))
    (:`NewEnumerator1`
      (bind _output_get_2 (set `local.Spawn Right Problem` (`KismetMathLibrary.RandomBool`)))
      (if _output_get_2
        (`|SpawnActorFromClass` "/Game/Blueprints/MathProblem_UI.MathProblem_UI_C" (`SceneComponent.K2_GetComponentToWorld` (`self.Right Segment Right side Math Problem Box collision`)) "Undefined" "MultiplyWithRoot" null null)))
    (:`NewEnumerator2`
      (bind _output_get_3 (set `local.Spawn Forward Problem` (`KismetMathLibrary.RandomBool`)))
      (if _output_get_3
        (`|SpawnActorFromClass` "/Game/Blueprints/MathProblem_UI.MathProblem_UI_C" (`SceneComponent.K2_GetComponentToWorld` (`self.Forward  Math Problem Box collision`)) "Undefined" "MultiplyWithRoot" null null)))))

(fn `Decide What Segment To Do Next`
  (bind _possible_directions (`self.Possible Directions`))
  (bind _returnvalue (`KismetArrayLibrary.Array_Length` _possible_directions))
  (`|ExecutionSequence`
    (:`then_0`
      (bind _returnvalue_2 (`self.Calculate Forward location and Rotation`))
      (if (or (>= (.x _returnvalue_2) 76800.0) (>= (.y _returnvalue_2) 76800.0))
        (`KismetSystemLibrary.PrintString` "Forward would have gone out of Bounds" true true (struct :`R` 1.0 :`G` 0.903147 :`A` 1.0) 10.0)
        (else
          (`KismetArrayLibrary.Array_Add` (`self.Possible Directions`) "NewEnumerator2"))))
    (:`then_1`
      (bind _returnvalue_3 (`self.Calculate Left Location and Rotation`))
      (if (or (>= (.x _returnvalue_3) 76800.0) (>= (.y _returnvalue_3) 76800.0))
        (`KismetSystemLibrary.PrintString` "Left would have gone out of Bounds" true true (struct :`R` 1.0 :`G` 0.902361 :`A` 1.0) 10.0)
        (else
          (`KismetArrayLibrary.Array_Add` (`self.Possible Directions`) "NewEnumerator0"))))
    (:`then_2`
      (bind _returnvalue_4 (`self.Calculate Right Location and Rotation`))
      (if (or (>= (.x _returnvalue_4) 76800.0) (>= (.y _returnvalue_4) 76800.0))
        (`KismetSystemLibrary.PrintString` "Right would have gone out of Bounds" true true (struct :`R` 1.0 :`G` 0.945208 :`A` 1.0) 10.0)
        (else
          (`KismetArrayLibrary.Array_Add` (`self.Possible Directions`) "NewEnumerator1"))))
    (:`then_3`
      (if (> _returnvalue 0)
        (bind _output_get (set `self.Turn directions ref` (`|GetArrayItem` _possible_directions (`KismetMathLibrary.RandomIntegerInRange` 0 (- _returnvalue 1)))))
        (switch `/Game/Blueprints/Turn_Directions` _output_get
          (:`NewEnumerator0`
            (`self.Setup Turn Direction`))
          (:`NewEnumerator1`
            (`self.Setup Turn Direction`))
          (:`NewEnumerator2`
            (set `PrimitiveComponent.bGenerateOverlapEvents` false (`self.Turn box`))
            (`self.Set up Forward Direction`)))))))

(fn `Set up Forward Direction`
  (bind _left_segment_leftfloor (`self.Left Segment Leftfloor`))
  (bind _left_segment_right_wall_right_side (`self.Left Segment Right Wall Right side`))
  (bind _left_segment_leftwall_left_side (`self.Left Segment Leftwall left side`))
  (bind _right_segment_right_floor (`self.Right Segment Right Floor`))
  (bind _right_segment_rightfllor_right_side (`self.Right Segment Rightfllor Right Side`))
  (bind _right_segment__left_wall_left_side (`self.Right Segment  Left wall left side`))
  (`SceneComponent.SetVisibility` (`self.Cube`) false false)
  (`SceneComponent.SetVisibility` (`self.Forward connector`) true true)
  (`PrimitiveComponent.SetCollisionEnabled` (`self.Forward_Left_wall_connector`) "QueryAndPhysics")
  (`PrimitiveComponent.SetCollisionEnabled` (`self.Forward_right_wall_connector`) "QueryAndPhysics")
  (`|ExecutionSequence`
    (:`then_0`
      (`|ExecutionSequence`
        (:`then_0`
          (`SceneComponent.SetVisibility` _left_segment_leftfloor false false)
          (`SceneComponent.SetVisibility` _left_segment_right_wall_right_side false false)
          (`SceneComponent.SetVisibility` _left_segment_leftwall_left_side false false))
        (:`then_1`
          (`PrimitiveComponent.SetCollisionEnabled` _left_segment_leftfloor "NoCollision")
          (`PrimitiveComponent.SetCollisionEnabled` _left_segment_right_wall_right_side "NoCollision")
          (`PrimitiveComponent.SetCollisionEnabled` _left_segment_leftwall_left_side "QueryAndPhysics"))))
    (:`then_1`
      (`|ExecutionSequence`
        (:`then_0`
          (`SceneComponent.SetVisibility` _right_segment_right_floor false false)
          (`SceneComponent.SetVisibility` _right_segment_rightfllor_right_side false false)
          (`SceneComponent.SetVisibility` _right_segment__left_wall_left_side false false))
        (:`then_1`
          (`PrimitiveComponent.SetCollisionEnabled` _right_segment_right_floor "QueryAndPhysics")
          (`PrimitiveComponent.SetCollisionEnabled` _right_segment_rightfllor_right_side "QueryAndPhysics")
          (`PrimitiveComponent.SetCollisionEnabled` _right_segment__left_wall_left_side "QueryAndPhysics"))))
    (:`then_2`
      (set `self.Turn directions ref` "NewEnumerator2"))
    (:`then_3`
      (`self.Decide to Spawn A math Problem` "NewEnumerator2"))))

(fn `Setup Turn Direction`
  (bind _left_segment_leftfloor (`self.Left Segment Leftfloor`))
  (bind _left_segment_right_wall_right_side (`self.Left Segment Right Wall Right side`))
  (bind _left_segment_leftwall_left_side (`self.Left Segment Leftwall left side`))
  (bind _right_segment_right_floor (`self.Right Segment Right Floor`))
  (bind _right_segment_rightfllor_right_side (`self.Right Segment Rightfllor Right Side`))
  (bind _right_segment__left_wall_left_side (`self.Right Segment  Left wall left side`))
  (bind _left_connector (`self.Left connector`))
  (bind _right_connector (`self.right connector`))
  (bind _returnvalue (`|SpawnActorFromClass` "/Game/Blueprints/Turn_Collision.Turn_Collision_C" (`SceneComponent.K2_GetComponentToWorld` (`self.Turn box`)) "Undefined" "MultiplyWithRoot" null null))
  (`BoxComponent.SetBoxExtent` (`/Game/Blueprints/Turn_Collision.Box` _returnvalue) (`BoxComponent.BoxExtent` (`self.Turn box`)) true)
  (switch `/Game/Blueprints/Turn_Directions` (`self.Turn directions ref`)
    (:`NewEnumerator0`
      (set `/Game/Blueprints/Turn_Collision.Left Or Right` "NewEnumerator0" _returnvalue)
      (`|ExecutionSequence`
        (:`then_0`
          (`SceneComponent.SetVisibility` _right_segment_right_floor false false)
          (`SceneComponent.SetVisibility` _right_segment_rightfllor_right_side false false)
          (`SceneComponent.SetVisibility` _right_segment__left_wall_left_side false false)
          (`SceneComponent.SetVisibility` _left_connector true true))
        (:`then_1`
          (`PrimitiveComponent.SetCollisionEnabled` _right_segment_right_floor "NoCollision")
          (`PrimitiveComponent.SetCollisionEnabled` _right_segment_rightfllor_right_side "NoCollision")
          (`PrimitiveComponent.SetCollisionEnabled` _right_segment__left_wall_left_side "NoCollision")
          (`PrimitiveComponent.SetCollisionEnabled` _left_connector "NoCollision")
          (`PrimitiveComponent.SetCollisionEnabled` (`self.Left_Cnnector_wall_connector`) "QueryAndPhysics")
          (`PrimitiveComponent.SetCollisionEnabled` (`self.Left_Cnnector_wall_connector2`) "QueryAndPhysics"))
        (:`then_2`
          (set `self.Turn directions ref` "NewEnumerator0"))
        (:`then_3`
          (`self.Decide to Spawn A math Problem` "NewEnumerator0"))))
    (:`NewEnumerator1`
      (set `/Game/Blueprints/Turn_Collision.Left Or Right` "NewEnumerator1" _returnvalue)
      (`|ExecutionSequence`
        (:`then_0`
          (`SceneComponent.SetVisibility` _left_segment_leftfloor false false)
          (`SceneComponent.SetVisibility` _left_segment_right_wall_right_side false false)
          (`SceneComponent.SetVisibility` _left_segment_leftwall_left_side false false)
          (`SceneComponent.SetVisibility` _right_connector true true))
        (:`then_1`
          (`PrimitiveComponent.SetCollisionEnabled` _left_segment_leftfloor "NoCollision")
          (`PrimitiveComponent.SetCollisionEnabled` _left_segment_right_wall_right_side "NoCollision")
          (`PrimitiveComponent.SetCollisionEnabled` _left_segment_leftwall_left_side "NoCollision")
          (`PrimitiveComponent.SetCollisionEnabled` _right_connector "NoCollision")
          (`PrimitiveComponent.SetCollisionEnabled` (`self.Right_connector_left_wall_connector`) "QueryAndPhysics")
          (`PrimitiveComponent.SetCollisionEnabled` (`self.Right_connector_front_wall_connector`) "QueryAndPhysics"))
        (:`then_2`
          (set `self.Turn directions ref` "NewEnumerator1"))
        (:`then_3`
          (`self.Decide to Spawn A math Problem` "NewEnumerator1"))))))

(fn `Spawn Cross Section at Right End`
  (if (`/Game/Blueprints/BP_ProceduralBuilder.SpawnEndGoal?` (`self.Builder REF`))
    (set `self.Gap value` 2100.0)
    (bind (_returnvalue _returnvalue_roll _returnvalue_pitch _returnvalue2) (`self.Calculate Right Location and Rotation`))
    (`|SpawnActorFromClass` "/Game/Blueprints/BP_Level3_Endgoal.BP_Level3_Endgoal_C" (`KismetMathLibrary.MakeTransform` _returnvalue (`KismetMathLibrary.MakeRotator` _returnvalue_roll _returnvalue_pitch _returnvalue2)) "Undefined" "MultiplyWithRoot" null null)
    (else
      (bind (_returnvalue_2 _returnvalue_roll_2 _returnvalue_pitch_2 _returnvalue2_2) (`self.Calculate Right Location and Rotation`))
      (bind _returnvalue_3 (`|SpawnActorFromClass` (`GameplayStatics.GetObjectClass` self) (`KismetMathLibrary.MakeTransform` (- _returnvalue_2 (`self.Offset`)) (`KismetMathLibrary.MakeRotator` _returnvalue_roll_2 _returnvalue_pitch_2 _returnvalue2_2)) "Undefined" "MultiplyWithRoot" null null))
      (`/Game/Blueprints/BP_ProceduralBuilder.Add to Segments` (`self.Builder REF`) _returnvalue_3))))

(fn `Spawn Cross Section at the Forward end`
  (if (`/Game/Blueprints/BP_ProceduralBuilder.SpawnEndGoal?` (`self.Builder REF`))
    (set `self.Gap value` 2100.0)
    (bind (_returnvalue _returnvalue2) (`self.Calculate Forward location and Rotation`))
    (`|SpawnActorFromClass` "/Game/Blueprints/BP_Level3_Endgoal.BP_Level3_Endgoal_C" (`KismetMathLibrary.MakeTransform` _returnvalue _returnvalue2) "Undefined" "MultiplyWithRoot" null null)
    (else
      (bind (_returnvalue_2 _returnvalue2_2) (`self.Calculate Forward location and Rotation`))
      (bind _returnvalue_3 (`|SpawnActorFromClass` (`GameplayStatics.GetObjectClass` self) (`KismetMathLibrary.MakeTransform` (- _returnvalue_2 (`self.Offset`)) _returnvalue2_2) "Undefined" "MultiplyWithRoot" null null))
      (`/Game/Blueprints/BP_ProceduralBuilder.Add to Segments` (`self.Builder REF`) _returnvalue_3))))

(fn `Spawn Cross section at the Left End`
  (if (`/Game/Blueprints/BP_ProceduralBuilder.SpawnEndGoal?` (`self.Builder REF`))
    (set `self.Gap value` 2100.0)
    (bind (_returnvalue _returnvalue_roll _returnvalue_pitch _returnvalue2) (`self.Calculate Left Location and Rotation`))
    (`|SpawnActorFromClass` "/Game/Blueprints/BP_Level3_Endgoal.BP_Level3_Endgoal_C" (`KismetMathLibrary.MakeTransform` _returnvalue (`KismetMathLibrary.MakeRotator` _returnvalue_roll _returnvalue_pitch _returnvalue2)) "Undefined" "MultiplyWithRoot" null null)
    (else
      (bind (_returnvalue_2 _returnvalue_roll_2 _returnvalue_pitch_2 _returnvalue2_2) (`self.Calculate Left Location and Rotation`))
      (bind _returnvalue_3 (`|SpawnActorFromClass` (`GameplayStatics.GetObjectClass` self) (`KismetMathLibrary.MakeTransform` (- _returnvalue_2 (`self.Offset`)) (`KismetMathLibrary.MakeRotator` _returnvalue_roll_2 _returnvalue_pitch_2 _returnvalue2_2)) "Undefined" "MultiplyWithRoot" null null))
      (`/Game/Blueprints/BP_ProceduralBuilder.Add to Segments` (`self.Builder REF`) _returnvalue_3))))

(fn `UserConstructionScript`)
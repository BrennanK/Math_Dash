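; Tutorial trigger box that pauses player movement to show instruction text and an optional looping video.
; On player overlap it snaps the pawn to itself, swaps to a no-movement input context, blends the view to itself and opens Tutorial_Widget.
; ChangeCameraBack turns the pawn via a spawned Turn_Collision, then restores camera and input, optionally spawning BP_Teacher.
; When media plays, PreviousPathBox also starts blocking pawns.
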(event `self.Box.OnComponentBeginOverlap`
  (params (OverlappedComponent :type "PrimitiveComponent Object Reference") (OtherActor :type "Actor Object Reference") (OtherComp :type "PrimitiveComponent Object Reference") (OtherBodyIndex :type Integer) (bFromSweep :type Boolean) (SweepResult :type "HitResult Structure (by ref)"))
  (bind _returnvalue (`GameplayStatics.GetPlayerPawn` 0))
  (if (== OtherActor (`GameplayStatics.GetPlayerPawn` 0))
    (`self.Display Video and Txet`)
    (`self.Disable Player IMC`)
    (message `/Game/Blueprints/BPI_PlayerCharacter.Set Teacher Distance from Player` _returnvalue 0.0)
    (`self.K2_SetActorLocation` _returnvalue (+ (`self.K2_GetActorLocation`) (0.0 0.0 60.0)) false false)))

(event `Display Video and Txet`
  (bind _media_player_for_video (`self.Media Player for Video`))
  (if (== (`self.Trigger UI Reveal Index`) 0.0)
    (set `self.Trigger UI Reveal Index` (`KismetMathLibrary.Conv_IntToDouble` (- (`KismetArrayLibrary.Array_Length` (`self.Instruction String`)) 1))))
  (`PlayerController.SetViewTargetWithBlend` (`GameplayStatics.GetPlayerController` 0) self (`self.Blend Time`) "VTBlend_Linear" 0.0 false)
  (bind _returnvalue (`|CreateWidget` "/Game/Widgets/Tutorial_Widget.Tutorial_Widget_C"))
  (bind _output_get (set `self.Tut Widget Ref` _returnvalue))
  (set `/Game/Widgets/Tutorial_Widget.Teach Box Ref` self _output_get)
  (`UserWidget.AddToViewport` _returnvalue 0)
  (`UserWidget.AddToViewport` _output_get 0)
  (`WidgetBlueprintLibrary.SetInputMode_GameAndUIEx` (`GameplayStatics.GetPlayerController` 0) (`self.Tut Widget Ref`))
  (`/Game/Widgets/Tutorial_Widget.Set New Instructions Text` (`self.Tut Widget Ref`) (`|GetArrayItem` (`self.Instruction String`)))
  (`KismetSystemLibrary.Delay` (`self.Blend Time`))
  (if (`self.Play Media?`)
    (`MediaPlayer.OpenSource` _media_player_for_video (`self.Media Source`))
    (`MediaPlayer.SetLooping` _media_player_for_video true)
    (`MediaPlayer.Play` _media_player_for_video)
    (`PrimitiveComponent.SetCollisionResponseToChannel` (`self.Previous Path Box`) "ECC_Pawn" "ECR_Block")))

(event `Change Camera Back`
  (bind _returnvalue (`GameplayStatics.GetPlayerPawn` 0))
  (bind _blend_time (`self.Blend Time`))
  (`KismetSystemLibrary.PrintString` "Change Camera called")
  (bind _returnvalue_2 (`|SpawnActorFromClass` "/Game/Blueprints/Turn_Collision.Turn_Collision_C" (`self.GetTransform`) "Undefined" "MultiplyWithRoot" null null))
  (set `self.Delay Before IMC change` (`/Game/Blueprints/Turn_Collision.Lerp Time` _returnvalue_2))
  (set `/Game/Blueprints/Turn_Collision.Left Or Right` (`self.Direction to Turn`) _returnvalue_2)
  (`/Game/Blueprints/Turn_Collision.Initiate Rotation` _returnvalue_2 (`GameplayStatics.GetPlayerPawn` 0))
  (`KismetSystemLibrary.Delay` (`self.Delay Before IMC change`))
  (`PlayerController.SetViewTargetWithBlend` (`GameplayStatics.GetPlayerController` 0) (`GameplayStatics.GetPlayerPawn` 0) _blend_time "VTBlend_Linear" 0.0 false)
  (`KismetSystemLibrary.Delay` _blend_time)
  (bind _asplayer_controller (cast `PlayerController` (`Pawn.GetController` (`GameplayStatics.GetPlayerPawn` 0))))
  (bind _returnvalue_3 (pcsubsystem `EnhancedInputLocalPlayerSubsystem` _asplayer_controller))
  (`/Engine/EditorBlueprintResources/StandardMacros.IsValid` _returnvalue_3
    (:`Is Valid`
      (`EnhancedInputSubsystemInterface.RemoveMappingContext` _returnvalue_3 "/Game/ThirdPerson/Input/No_Movement_IMC.No_Movement_IMC" (struct))
      (`EnhancedInputSubsystemInterface.AddMappingContext` _returnvalue_3 "/Game/ThirdPerson/Input/IMC_Default.IMC_Default" 0 (struct))
      (`WidgetBlueprintLibrary.SetInputMode_GameOnly` (`GameplayStatics.GetPlayerController` 0) true)
      (if (`self.Spawn Teacher?`)
        (`|SpawnActorFromClass` "/Game/Blueprints/BP_Teacher.BP_Teacher_C" (`KismetMathLibrary.MakeTransform` (`self.Teacher Spawn Location`)) "Undefined" "MultiplyWithRoot" null null)
        (message `/Game/Blueprints/BPI_PlayerCharacter.Set Teacher ref` _returnvalue)
        (message `/Game/Blueprints/BPI_PlayerCharacter.Set Teacher Distance from Player` (`GameplayStatics.GetPlayerPawn` 0) 2.5)
        (bind _turn_collision_ref (message `/Game/Blueprints/BPI_PlayerCharacter.Get Turn Collision Ref` _returnvalue))
        (`KismetArrayLibrary.Array_Clear` _turn_collision_ref)
        (`KismetSystemLibrary.PrintString` (`KismetStringLibrary.Concat_StrStr` "Turn collision ref length is " (`KismetStringLibrary.Conv_IntToString` (`KismetArrayLibrary.Array_Length` _turn_collision_ref))))))))

(fn `Disable Player IMC`
  (bind _asplayer_controller (cast `PlayerController` (`Pawn.GetController` (`GameplayStatics.GetPlayerPawn` 0))))
  (bind _returnvalue (pcsubsystem `EnhancedInputLocalPlayerSubsystem` _asplayer_controller))
  (`/Engine/EditorBlueprintResources/StandardMacros.IsValid` _returnvalue
    (:`Is Valid`
      (`EnhancedInputSubsystemInterface.RemoveMappingContext` _returnvalue "/Game/ThirdPerson/Input/IMC_Default.IMC_Default" (struct))
      (`EnhancedInputSubsystemInterface.AddMappingContext` _returnvalue "/Game/ThirdPerson/Input/No_Movement_IMC.No_Movement_IMC" 0 (struct)))))

(fn `UserConstructionScript`)
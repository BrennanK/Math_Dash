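; MathProblem_Gate is a gate Blueprint made of eight wall sections in two rows of four, one of which is randomly picked as the trigger spot.
; On BeginPlay it gives the chosen section a different material and offsets the Box collision to that grid position using the section index.
; When a BP_ThirdPersonCharacter overlaps the Box, it sets the TouchedMultiplierGate flag.
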(event `self.ReceiveBeginPlay`
  (bind _box (`self.Box`))
  (bind _box_2 (`self.Box`))
  (bind _array (`|MakeArray` (`self.Transparent_Section_1`) (`self.Transparent_Section_2`) (`self.Transparent_Section_3`) (`self.Transparent_Section_4`) (`self.Transparent_Section_5`) (`self.Transparent_Section_6`) (`self.Transparent_Section_7`) (`self.Transparent_Section_8`)))
  (set `self.Generated Index` (`KismetMathLibrary.RandomIntegerInRange` 0 (- (`KismetArrayLibrary.Array_Length` _array) 1)))
  (for (_array_element _array_index) _array
    (if (== _array_index (`self.Generated Index`))
      (`PrimitiveComponent.SetMaterial` _array_element 0 "/Game/Imports/Props/Transparent_wall/Inst_tr_wall1.Inst_tr_wall1")
      (if (> _array_index 3)
        (`SceneComponent.K2_SetRelativeLocation` _box (+ (`SceneComponent.RelativeLocation` _box) (`KismetMathLibrary.MakeVector` 0.0 (* (- _array_index 4) 135.0) 300.0)) false false)
        (else
          (`SceneComponent.K2_SetRelativeLocation` _box_2 (+ (`SceneComponent.RelativeLocation` _box_2) (`KismetMathLibrary.MakeVector` 0.0 (* _array_index 135.0))) false false))))))

(event `self.Box.OnComponentBeginOverlap`
  (params (OverlappedComponent :type "PrimitiveComponent Object Reference") (OtherActor :type "Actor Object Reference") (OtherComp :type "PrimitiveComponent Object Reference") (OtherBodyIndex :type Integer) (bFromSweep :type Boolean) (SweepResult :type "HitResult Structure (by ref)"))
  (cast `/Game/ThirdPerson/Blueprints/BP_ThirdPersonCharacter` OtherActor)
  (set `self.Touched Multiplier Gate` true))

(fn `UserConstructionScript`)